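; BP_Ceiling is a ceiling Blueprint with an emissive glow that can be dimmed through its Dim event.
; The construction script gives the Cube a dynamic instance of MI_Ceiling and sets a bright white EmissionTint.
; Dim captures the current tint, then plays a timeline whose BrightnessFactor blends EmissionTint between black and that captured color.
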(event `Dim`
  (bind _returnvalue (`MaterialInstanceDynamic.K2_GetVectorParameterValue` (`self.Material`) "EmissionTint"))
  (bind (_direction _brightnessfactor) (`Timeline|DimTimeline` :!via `PlayFromStart`)
    (:`Update`
      (`MaterialInstanceDynamic.SetVectorParameterValue` (`self.Material`) "EmissionTint" (`KismetMathLibrary.LinearColorLerp` (struct :`A` 1.0) _returnvalue _brightnessfactor)))))

(fn `UserConstructionScript`
  (bind _returnvalue (`PrimitiveComponent.CreateDynamicMaterialInstance` (`self.Cube`) 0 "/Game/BLAQ/Assets/Ceiling/MI_Ceiling.MI_Ceiling" "None"))
  (bind _output_get (set `self.Material` _returnvalue))
  (`MaterialInstanceDynamic.SetVectorParameterValue` _output_get "EmissionTint" (struct :`R` 5.0 :`G` 5.0 :`B` 5.0 :`A` 1.0)))