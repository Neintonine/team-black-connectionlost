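; BP_MainMenu_Enemy is an enemy for the main menu that can be switched in and out of a chase state.
; SetChase writes the ChasePlayer bool to its AI controller's blackboard, acting only when the value differs from the stored one.
; On a change it crossfades audio, playing either the monster chase or default sound and fading the other out.
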(fn `SetChase`
  (params (BoolValue :type Boolean))
  (bind _audio_default (`self.Audio_Default`))
  (bind _audio_monsterchase (`self.Audio_MonsterChase`))
  (bind _returnvalue (`AIBlueprintHelperLibrary.GetBlackboard` (`AIBlueprintHelperLibrary.GetAIController` self)))
  (if (not (== (`BlackboardComponent.GetValueAsBool` _returnvalue "ChasePlayer") BoolValue))
    (`BlackboardComponent.SetValueAsBool` _returnvalue "ChasePlayer" BoolValue)
    (`AudioComponent.Play` (select `bool` BoolValue :`false` _audio_default :`true` _audio_monsterchase) 0.0)
    (`AudioComponent.FadeOut` (select `bool` BoolValue :`false` _audio_monsterchase :`true` _audio_default) 0.5 0.0 "Linear")))

(fn `UserConstructionScript`)