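; BP_MainMenuPawn is the pawn that runs the main menu.
; On BeginPlay it has the first player controller possess it, opens the non-pausing main menu, stores the widget, plays the menu music and switches the base sound mix to the menu mix.
; On EndPlay it closes the stored menu widget and sets the base sound mix to the master mix.
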(event `self.ReceiveBeginPlay`
  (`Controller.Possess` (`GameplayStatics.GetPlayerController` 0) self)
  (bind _widget (`/Game/BLAQ/Blueprints/MainMenu/BPFL_MainMenuFunctions.OpenMainMenu` 0 false))
  (set `self.Widget` _widget)
  (`GameplayStatics.PlaySound2D` "/Game/Devs/Luca/DevLevel/Sound/Menu_Music.Menu_Music" 1.0 1.0 0.0 "/Game/Devs/Luca/DevLevel/Sound/PlaySingle.PlaySingle" self)
  (`GameplayStatics.SetBaseSoundMix` "/Game/Devs/Luca/DevLevel/Sound/SoundMixers/SCM_MenuMusic.SCM_MenuMusic"))

(event `self.ReceiveEndPlay`
  (params (EndPlayReason :type "EEndPlayReason Enum" :default "Destroyed"))
  (`/Game/BLAQ/Blueprints/MainMenu/BPFL_MainMenuFunctions.CloseMainMenu` (`self.Widget`))
  (`GameplayStatics.SetBaseSoundMix` "/Game/Devs/Luca/DevLevel/Sound/SoundMixers/SCM_Master.SCM_Master"))

(fn `UserConstructionScript`)