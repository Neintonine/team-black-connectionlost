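; Main menu display actor that shows a randomly chosen object with a gentle floating motion.
; On BeginPlay it spawns a random class from ViableObjects at the DisplayArrow transform and attaches it to that arrow, keeping world transform.
; Each Tick drives the arrow's relative Z with a sine of game time, so the attached object bobs along with it.
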(event `self.ReceiveBeginPlay`
  (bind _returnvalue (`|SpawnActorFromClass` (`KismetArrayLibrary.Array_Random` (`self.ViableObjects`)) (`SceneComponent.K2_GetComponentToWorld` (`self.DisplayArrow`)) "Undefined" "MultiplyWithRoot" self null))
  (`self.K2_AttachToComponent` _returnvalue (`self.DisplayArrow`) "None" "KeepWorld" "KeepWorld" "KeepWorld" true))

(event `self.ReceiveTick`
  (params (DeltaSeconds :type "Float (single-precision)"))
  (`SceneComponent.K2_SetRelativeLocation` (`self.DisplayArrow`) (`KismetMathLibrary.MakeVector` 0.0 0.0 (* (`KismetMathLibrary.Sin` (* (`GameplayStatics.GetTimeSeconds`) 1.0)) 2.0)) false false))

(fn `UserConstructionScript`)