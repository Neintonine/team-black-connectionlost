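; BP_EnemyAI is the monster enemy character that chases the first-person player and kills them on contact.
; Pawn sensing starts a chase when allowed, and Tick ends it once the player is beyond LooseDistance.
; SetChase drives the blackboard ChasePlayer key unless StayStill is set, crossfading chase and default audio.
; A sphere overlap triggers the player's Death and unpossesses the enemy, and overlapping BP_Arcade actors dim their lights until it leaves.
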(event `self.ReceiveTick`
  (params (DeltaSeconds :type "Float (single-precision)"))
  (bind _returnvalue (`GameplayStatics.GetPlayerCharacter` 0))
  (`/Engine/EditorBlueprintResources/StandardMacros.IsValid` _returnvalue
    (:`Is Valid`
      (if (> (`KismetMathLibrary.Vector_Distance` (`SceneComponent.K2_GetComponentLocation` (`Character.CapsuleComponent` _returnvalue)) (`SceneComponent.K2_GetComponentLocation` (`self.CapsuleComponent`))) (`self.LooseDistance`))
        (`self.SetChase` false)))))

(event `self.ReceiveActorEndOverlap`
  (params (OtherActor :type "Actor Object Reference"))
  (bind _asbp_arcade (cast `/Game/BLAQ/Assets/Arcade-Machine/BP_Arcade` OtherActor))
  (`/Game/BLAQ/Assets/Arcade-Machine/BP_Arcade.BrightenLights` _asbp_arcade))

(event `self.ReceiveActorBeginOverlap`
  (params (OtherActor :type "Actor Object Reference"))
  (bind _asbp_arcade (cast `/Game/BLAQ/Assets/Arcade-Machine/BP_Arcade` OtherActor))
  (`/Game/BLAQ/Assets/Arcade-Machine/BP_Arcade.DimLights` _asbp_arcade))

(event `self.PawnSensing.OnSeePawn`
  (params (Pawn :type "Pawn Object Reference"))
  (if (`self.AllowSensingPlayer`)
    (cast `/Game/FirstPerson/Blueprints/BP_FirstPersonCharacter` Pawn)
    (`self.SetChase` true)))

(event `self.Sphere.OnComponentBeginOverlap`
  (params (OverlappedComponent :type "PrimitiveComponent Object Reference") (OtherActor :type "Actor Object Reference") (OtherComp :type "PrimitiveComponent Object Reference") (OtherBodyIndex :type Integer) (bFromSweep :type Boolean) (SweepResult :type "HitResult Structure (by ref)"))
  (bind _asbp_first_person_character (cast `/Game/FirstPerson/Blueprints/BP_FirstPersonCharacter` OtherActor))
  (`/Game/FirstPerson/Blueprints/BP_FirstPersonCharacter.Death` _asbp_first_person_character self)
  (`Controller.UnPossess` (`self.GetController`)))

(fn `SetChase`
  (params (BoolValue :type Boolean))
  (bind _audio_default (`self.Audio_Default`))
  (bind _audio_monsterchase (`self.Audio_MonsterChase`))
  (bind _returnvalue (`AIBlueprintHelperLibrary.GetBlackboard` (`AIBlueprintHelperLibrary.GetAIController` self)))
  (if (`BlackboardComponent.GetValueAsBool` _returnvalue "StayStill")
    _
    (elif (not (== (`BlackboardComponent.GetValueAsBool` _returnvalue "ChasePlayer") BoolValue))
      (`BlackboardComponent.SetValueAsBool` _returnvalue "ChasePlayer" BoolValue)
      (`AudioComponent.Play` (select `bool` BoolValue :`false` _audio_default :`true` _audio_monsterchase) 0.0)
      (`AudioComponent.FadeOut` (select `bool` BoolValue :`false` _audio_monsterchase :`true` _audio_default) 0.5 0.0 "Linear"))))

(fn `UserConstructionScript`)