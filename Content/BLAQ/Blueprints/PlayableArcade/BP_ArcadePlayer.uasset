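; BP_ArcadePlayer is the pawn for a playable arcade machine minigame, possessed while the first-person character stays the view target.
; It adds its own input mapping for exiting the arcade, and forwards pause to the first-person character's menu.
; Setup links the arcade machine and commands spawners to spawn the current level.
; Completing a level advances the machine and respawns, while failing exits with a timeout and plays a sound.
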(event `self.ReceiveBeginPlay`
  (bind _returnvalue (`GameplayStatics.GetPlayerController` 0))
  (bind _returnvalue_2 (`GameplayStatics.GetActorOfClass` "/Game/FirstPerson/Blueprints/BP_FirstPersonCharacter.BP_FirstPersonCharacter_C"))
  (set `self.ActualPlayerCharacter` _returnvalue_2)
  (`Controller.Possess` _returnvalue self)
  (`PlayerController.SetViewTargetWithBlend` _returnvalue (`self.ActualPlayerCharacter`) 0.0 "VTBlend_Linear" 0.0 false)
  (`KismetSystemLibrary.Delay` 0.2)
  (`EnhancedInputSubsystemInterface.AddMappingContext` (pcsubsystem `EnhancedInputLocalPlayerSubsystem` (`GameplayStatics.GetPlayerController` 0)) (`self.InputMapping`) 0 (struct)))

(event `EnhancedInput|/Game/BLAQ/Input/Actions/IA_ExitArcade`
  (params (ActionValue :type Boolean) (ElapsedSeconds :type "Float (double-precision)") (TriggeredSeconds :type "Float (double-precision)") (InputAction :type "InputAction Object Reference" :default "/Game/BLAQ/Input/Actions/IA_ExitArcade.IA_ExitArcade"))
  (:`Triggered`
    (`/Game/BLAQ/Blueprints/PlayableArcade/BP_PlayableArcade.ExitArcade` (`self.ArcadeMachine`) false "NewEnumerator0")))

(event `EnhancedInput|/Game/FirstPerson/Input/Actions/IA_PauseGame`
  (params (ActionValue :type Boolean) (ElapsedSeconds :type "Float (double-precision)") (TriggeredSeconds :type "Float (double-precision)") (InputAction :type "InputAction Object Reference" :default "/Game/FirstPerson/Input/Actions/IA_PauseGame.IA_PauseGame"))
  (:`Started`
    (`/Game/FirstPerson/Blueprints/BP_FirstPersonCharacter.HandleMainMenuInput` (`self.ActualPlayerCharacter`))))

(fn `_IssueSpawnCommand`
  (params (Reason :type "/Game/BLAQ/Blueprints/PlayableArcade/BPE_ArcadeSpawnReason Enum" :default "NewEnumerator0"))
  (for _array_element (`self.Spawners`)
    (`/Game/BLAQ/Blueprints/PlayableArcade/BP_ArcadeSpawner.Spawn` _array_element (`/Game/BLAQ/Blueprints/PlayableArcade/BP_PlayableArcade.CurrentLevel` (`self.ArcadeMachine`)) Reason)))

(fn `CompleteLevel`
  (`/Game/BLAQ/Blueprints/PlayableArcade/BP_PlayableArcade.CompleteLevel` (`self.ArcadeMachine`))
  (`self._IssueSpawnCommand` "NewEnumerator1"))

(fn `FailLevel`
  (`/Game/BLAQ/Blueprints/PlayableArcade/BP_PlayableArcade.ExitArcade` (`self.ArcadeMachine`) true "NewEnumerator0")
  (`self.PlaySound` "/Game/BLAQ/Sound/A_ArcadeFail_Cue.A_ArcadeFail_Cue"))

(fn `PlaySound`
  (params (Sound :type "SoundBase Object Reference"))
  (`GameplayStatics.PlaySoundAtLocation` Sound (`SceneComponent.K2_GetComponentLocation` (`/Game/FirstPerson/Blueprints/BP_FirstPersonCharacter.FirstPersonCamera` (`self.ActualPlayerCharacter`))) (struct) 1.0 1.0 0.0 null null null null)
  (return))

(fn `Setup`
  (params (ArcadeMachine :type "/Game/BLAQ/Blueprints/PlayableArcade/BP_PlayableArcade Object Reference"))
  (set `self.ArcadeMachine` ArcadeMachine)
  (`self._IssueSpawnCommand` "NewEnumerator0"))

(fn `UserConstructionScript`)