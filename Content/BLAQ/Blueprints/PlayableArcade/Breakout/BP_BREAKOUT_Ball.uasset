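; Ball for the Breakout arcade game, launched along -Y at a slight random angle and moved each Tick by a swept offset rather than physics.
; Blocking hits flip its X or Y direction from the impact normal, then branch on the hit actor.
; Targets notify the TargetSpawner, the death zone fails the player's level, and top paddle hits steer by offset from paddle center.
; Hits play target, paddle or wall sounds.
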(event `self.ReceiveBeginPlay`
  (set `self.MovementDirection` (`KismetMathLibrary.Normal` (`KismetMathLibrary.MakeVector` (`KismetMathLibrary.RandomFloatInRange` -0.5 0.5) -1.0))))

(event `self.ReceiveTick`
  (params (DeltaSeconds :type "Float (single-precision)"))
  (bind _sweephitresult (`SceneComponent.K2_AddWorldOffset` (`self.SphereCollision`) (* DeltaSeconds (`self.Speed`) (`self.MovementDirection`)) true false))
  (bind (_bblockinghit _binitialoverlap _time _distance _location _impactpoint _normal _impactnormal _physmat _hitactor) (`GameplayStatics.BreakHitResult` _sweephitresult))
  (if _bblockinghit
    (`self.HandleHitRegistration` _impactnormal _hitactor)))

(fn `HandleHitRegistration`
  (params (Normal :type "Vector Structure") (Actor :type "Actor Object Reference"))
  (bind (_movementdirection_x _movementdirection_y) (`KismetMathLibrary.BreakVector` (`self.MovementDirection`)))
  (bind _returnvalue_x (`KismetMathLibrary.BreakVector` (`SceneComponent.K2_GetComponentLocation` (`self.SphereCollision`))))
  (`|ExecutionSequence`
    (:`then_0`
      (if (> (`KismetMathLibrary.Abs` (.x Normal)) 0.1)
        (set `self.MovementDirection` (* (`self.MovementDirection`) (-1.0 1.0 1.0)))))
    (:`then_1`
      (if (> (`KismetMathLibrary.Abs` (.y Normal)) 0.1)
        (set `self.MovementDirection` (* (`self.MovementDirection`) (1.0 -1.0 1.0)))))
    (:`then_2`
      (bind _asbp_breakout_target (cast `/Game/BLAQ/Blueprints/PlayableArcade/Breakout/BP_BREAKOUT_Target` Actor))
      (`/Game/BLAQ/Blueprints/PlayableArcade/Breakout/BP_BREAKOUT_TargetSpawner.NotifyDestroy` (`self.TargetSpawner`) _asbp_breakout_target)
      (`/Game/BLAQ/Blueprints/PlayableArcade/BP_ArcadePlayer.PlaySound` (`self.Player`) "/Game/BLAQ/Sound/Breakout/A_BREAKOUT_BoxHit_Cue.A_BREAKOUT_BoxHit_Cue")
      (return))
    (:`then_3`
      (cast `/Game/BLAQ/Blueprints/PlayableArcade/Breakout/BP_BREAKOUT_DeathZone` Actor)
      (`/Game/BLAQ/Blueprints/PlayableArcade/BP_ArcadePlayer.FailLevel` (`self.Player`))
      (return))
    (:`then_4`
      (bind _asbp_breakout_player (cast `/Game/BLAQ/Blueprints/PlayableArcade/Breakout/BP_BREAKOUT_Player` Actor))
      (`/Game/BLAQ/Blueprints/PlayableArcade/BP_ArcadePlayer.PlaySound` _asbp_breakout_player "/Game/BLAQ/Sound/Breakout/A_BREAKOUT_PaddleHit_Cue.A_BREAKOUT_PaddleHit_Cue")
      (if (> (`KismetMathLibrary.Dot_VectorVector` Normal (0.0 -1.0 0.0)) 0.9)
        (bind _returnvalue_x_2 (`KismetMathLibrary.BreakVector` (`SceneComponent.K2_GetComponentLocation` (`/Game/BLAQ/Blueprints/PlayableArcade/BP_ArcadePlayer.DefaultSceneRoot` _asbp_breakout_player))))
        (bind _returnvalue_x_3 (`KismetMathLibrary.BreakVector` (`BoxComponent.GetScaledBoxExtent` (`/Game/BLAQ/Blueprints/PlayableArcade/Breakout/BP_BREAKOUT_Player.Box` _asbp_breakout_player))))
        (set `self.MovementDirection` (`KismetMathLibrary.Normal` (`KismetMathLibrary.MakeVector` (`KismetMathLibrary.Lerp` 0.0 0.75 (/ (- _returnvalue_x _returnvalue_x_2) _returnvalue_x_3)) _movementdirection_y)))
        (return)))
    (:`then_5`
      (`/Game/BLAQ/Blueprints/PlayableArcade/BP_ArcadePlayer.PlaySound` (`self.Player`) "/Game/BLAQ/Sound/Breakout/A_BREAKOUT_WallHit_Cue.A_BREAKOUT_WallHit_Cue"))))

(fn `UserConstructionScript`)