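; BP_BREAKOUT_TargetSpawner spawns and tracks the targets for the Breakout arcade game.
; Spawn reseeds a prefab collection randomly, loads the prefab, then gathers every BP_BREAKOUT_Target actor in the world into its list.
; NotifyDestroy removes and destroys a target, and tells the player to complete the level once the list is empty.
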(fn `NotifyDestroy`
  (params (`Target Object` :type "/Game/BLAQ/Blueprints/PlayableArcade/Breakout/BP_BREAKOUT_Target Object Reference"))
  (`KismetArrayLibrary.Array_RemoveItem` (`self.SpawnedTargets`) `Target Object`)
  (`self.K2_DestroyActor` `Target Object`)
  (if (< (`KismetArrayLibrary.Array_Length` (`self.SpawnedTargets`)) 1)
    (`/Game/BLAQ/Blueprints/PlayableArcade/BP_ArcadePlayer.CompleteLevel` (`self.Player`))))

(fn `Spawn`
  (params (Level :type Integer) (Reason :type "/Game/BLAQ/Blueprints/PlayableArcade/BPE_ArcadeSpawnReason Enum" :default "NewEnumerator0"))
  (bind _prefabcollection (`self.PrefabCollection`))
  (`PrefabActor.RandomizeSeed` _prefabcollection (`KismetMathLibrary.MakeRandomStream` (`KismetMathLibrary.RandomInteger` 10000000)) true)
  (`PrefabActor.LoadPrefab` _prefabcollection)
  (bind _outactors (`GameplayStatics.GetAllActorsOfClass` "/Game/BLAQ/Blueprints/PlayableArcade/Breakout/BP_BREAKOUT_Target.BP_BREAKOUT_Target_C"))
  (set `self.SpawnedTargets` _outactors))

(fn `UserConstructionScript`)