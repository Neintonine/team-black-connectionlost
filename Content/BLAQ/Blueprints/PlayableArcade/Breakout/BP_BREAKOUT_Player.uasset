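; BP_BREAKOUT_Player is the player-controlled piece in the playable Breakout arcade game, moved by the IA_BREAKOUT_Move Enhanced Input action.
; Each input event scales the axis value by PlayerSpeed, without delta time, and box-traces that step on the Visibility channel using the Box component's extent and rotation.
; If the trace hits nothing, the root teleports along world X by that step; otherwise it stays put.
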(event `EnhancedInput|/Game/BLAQ/Input/Actions/IA_BREAKOUT_Move`
  (params (ActionValue :type "Float (double-precision)") (ElapsedSeconds :type "Float (double-precision)") (TriggeredSeconds :type "Float (double-precision)") (InputAction :type "InputAction Object Reference" :default "/Game/BLAQ/Input/Actions/IA_BREAKOUT_Move.IA_BREAKOUT_Move"))
  (bind _box (`self.Box`))
  (bind _returnvalue (`SceneComponent.K2_GetComponentLocation` (`self.DefaultSceneRoot`)))
  (bind _returnvalue_2 (* ActionValue (`self.PlayerSpeed`)))
  (:`Triggered`
    (bind (_outhit _returnvalue_3) (`KismetSystemLibrary.BoxTraceSingle` _returnvalue (+ _returnvalue _returnvalue_2) (`BoxComponent.GetScaledBoxExtent` _box) (`SceneComponent.K2_GetComponentRotation` _box) "TraceTypeQuery1"))
    (if (not _returnvalue_3)
      (`SceneComponent.K2_AddWorldOffset` (`self.DefaultSceneRoot`) (`KismetMathLibrary.MakeVector` _returnvalue_2) false true))))

(fn `UserConstructionScript`
  (`parent.UserConstructionScript`))