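; Player pawn for the Hopper arcade minigame, hopping in grid steps sideways within fixed bounds or forward two cells on jump.
; Each hop plays a sound, and the move and jump inputs share a brief jumping-material swap on the visual mesh.
; Overlapping an obstacle, or standing over water detected by a per-tick downward trace, fails the level.
; Reaching a target completes the level, spawns a character copy there and resets to the origin.
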(event `self.ReceiveBeginPlay`
  (`parent.ReceiveBeginPlay`)
  (set `self.OriginPosition` (`SceneComponent.K2_GetComponentLocation` (`self.DefaultSceneRoot`)))
  (set `self.VisualCube` (`SceneComponent.GetChildComponent` (`SceneComponent.GetChildComponent` (`self.BP_HOPPER_PlayerCharacter`) 0) 0)))

(event `EnhancedInput|/Game/BLAQ/Input/Actions/IA_HOPPER_Move`
  (params (ActionValue :type "Vector2D Structure") (ElapsedSeconds :type "Float (double-precision)") (TriggeredSeconds :type "Float (double-precision)") (InputAction :type "InputAction Object Reference" :default "/Game/BLAQ/Input/Actions/IA_HOPPER_Move.IA_HOPPER_Move"))
  (bind _returnvalue (`KismetMathLibrary.SignOfFloat` ActionValue_X))
  (bind _returnvalue_x (`KismetMathLibrary.BreakVector` (`SceneComponent.K2_GetComponentLocation` (`self.DefaultSceneRoot`))))
  (bind _returnvalue_2 (* (`/Game/BLAQ/Blueprints/PlayableArcade/BP_Arcade_Definitions.GetGridSize`) _returnvalue))
  (:`Started`
    (`self.PlaySound` "/Game/BLAQ/Sound/Hopper/A_HOPPER_Jump_Cue.A_HOPPER_Jump_Cue")
    (`|ExecutionSequence`
      (:`then_1`
        (if (> (`KismetMathLibrary.Abs` ActionValue_X) 0.1)
          (if (< (`KismetMathLibrary.Abs` (+ _returnvalue_x _returnvalue_2)) 500.0)
            (`SceneComponent.K2_AddWorldOffset` (`self.DefaultSceneRoot`) (`KismetMathLibrary.MakeVector` _returnvalue_2) false false)
            (`self.K2_SetActorRotation` (`KismetMathLibrary.MakeRotator` 0.0 0.0 (* _returnvalue 90.0))))))
      (:`then_2`
        (bind _asstatic_mesh_component (cast `StaticMeshComponent` (`self.VisualCube`) :!label _label))
        (`PrimitiveComponent.SetMaterial` _asstatic_mesh_component 0 "/Game/BLAQ/Assets/Minigames/Hopper/MI_HOPPER_PlayerJumping.MI_HOPPER_PlayerJumping")
        (`KismetSystemLibrary.Delay` 0.2)
        (`PrimitiveComponent.SetMaterial` _asstatic_mesh_component 0 "/Game/BLAQ/Assets/Minigames/Hopper/MI_HOPPER_PlayerStanding.MI_HOPPER_PlayerStanding")))))

(event `EnhancedInput|/Game/BLAQ/Input/Actions/IA_HOPPER_Jump`
  (params (ActionValue :type Boolean) (ElapsedSeconds :type "Float (double-precision)") (TriggeredSeconds :type "Float (double-precision)") (InputAction :type "InputAction Object Reference" :default "/Game/BLAQ/Input/Actions/IA_HOPPER_Jump.IA_HOPPER_Jump"))
  (:`Started`
    (`self.PlaySound` "/Game/BLAQ/Sound/Hopper/A_HOPPER_Jump_Cue.A_HOPPER_Jump_Cue")
    (`SceneComponent.K2_AddWorldOffset` (`self.DefaultSceneRoot`) (`KismetMathLibrary.MakeVector` 0.0 (* (`/Game/BLAQ/Blueprints/PlayableArcade/BP_Arcade_Definitions.GetGridSize`) -2.0)) false false)
    (`self.K2_SetActorRotation` (`KismetMathLibrary.MakeRotator` 0.0))
    (goto _label)))

(event `self.ReceiveActorBeginOverlap`
  (params (OtherActor :type "Actor Object Reference"))
  (`|ExecutionSequence`
    (:`then_0`
      (cast `/Game/BLAQ/Blueprints/PlayableArcade/Hopper/Obstacles/BP_HOPPER_Obstacle` OtherActor)
      (`self.FailLevel`))
    (:`then_1`
      (bind _asbp_hopper_target (cast `/Game/BLAQ/Blueprints/PlayableArcade/Hopper/BP_HOPPER_Target` OtherActor))
      (`self.CompleteRun` _asbp_hopper_target))))

(event `self.ReceiveTick`
  (params (DeltaSeconds :type "Float (single-precision)"))
  (bind _returnvalue (`SceneComponent.K2_GetComponentLocation` (`self.DefaultSceneRoot`)))
  (bind (_outhit _returnvalue_2) (`KismetSystemLibrary.LineTraceSingle` _returnvalue (+ _returnvalue (* (`KismetMathLibrary.Vector_Up`) -350.0)) "TraceTypeQuery1"))
  (if _returnvalue_2
    (if (== (`GameplayStatics.GetObjectClass` (`.HitActor` (`GameplayStatics.BreakHitResult` _outhit))) "/Game/BLAQ/Blueprints/PlayableArcade/Hopper/BP_HOPPER_Water.BP_HOPPER_Water_C")
      (`self.FailLevel`))))

(fn `CompleteRun`
  (params (Target :type "/Game/BLAQ/Blueprints/PlayableArcade/Hopper/BP_HOPPER_Target Object Reference"))
  (`self.CompleteLevel`)
  (`|SpawnActorFromClass` "/Game/BLAQ/Blueprints/PlayableArcade/Hopper/BP_HOPPER_PlayerCharacter.BP_HOPPER_PlayerCharacter_C" (`KismetMathLibrary.MakeTransform` (`SceneComponent.K2_GetComponentLocation` (`self.BP_HOPPER_PlayerCharacter`)) (struct :`Yaw` 180.0)) "Undefined" "MultiplyWithRoot" Target null)
  (`SceneComponent.K2_SetWorldLocation` (`self.DefaultSceneRoot`) (`self.OriginPosition`) false false))

(fn `UserConstructionScript`
  (`parent.UserConstructionScript`))