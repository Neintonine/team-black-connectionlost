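; BP_HOPPER_Target is a target actor in the Hopper playable arcade game that spawns BP_HOPPER_PlayerCharacter instances.
; For one Reason value, Spawn creates as many characters as the Level, each owned by the target.
; They are placed at random X positions across its Box's width, on the box's Y, with a 180-degree rotation.
; On EndPlay it destroys any directly attached actors.
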(event `self.ReceiveEndPlay`
  (params (EndPlayReason :type "EEndPlayReason Enum" :default "Destroyed"))
  (for _array_element (`self.GetAttachedActors` true)
    (`self.K2_DestroyActor` _array_element)))

(fn `Spawn`
  (params (Level :type Integer) (Reason :type "/Game/BLAQ/Blueprints/PlayableArcade/BPE_ArcadeSpawnReason Enum" :default "NewEnumerator0"))
  (bind (_returnvalue_x _returnvalue_y) (`KismetMathLibrary.BreakVector` (`SceneComponent.K2_GetComponentLocation` (`self.Box`))))
  (bind _returnvalue_x_2 (`KismetMathLibrary.BreakVector` (`BoxComponent.GetScaledBoxExtent` (`self.Box`))))
  (if (`|EnumEquality` Reason "NewEnumerator0")
    (for _ (range Level)
      (`|SpawnActorFromClass` "/Game/BLAQ/Blueprints/PlayableArcade/Hopper/BP_HOPPER_PlayerCharacter.BP_HOPPER_PlayerCharacter_C" (`KismetMathLibrary.MakeTransform` (`KismetMathLibrary.MakeVector` (+ (`KismetMathLibrary.RandomFloatInRange` (* _returnvalue_x_2 -1.0) _returnvalue_x_2) _returnvalue_x) _returnvalue_y) (struct :`Yaw` 180.0)) "Undefined" "MultiplyWithRoot" self null))))

(fn `UserConstructionScript`)