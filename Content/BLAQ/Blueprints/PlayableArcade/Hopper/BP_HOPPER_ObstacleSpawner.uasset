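; Obstacle spawner for the Hopper arcade game that periodically spawns waves of moving obstacles.
; Each wave lines up random classes from a list behind an arrow component at a set offset, passing each obstacle its speed and spawner reference.
; A looping timer repeats waves, while the first wave spawns on BeginPlay and is nudged forward.
; EndPlay destroys remaining tracked obstacles and clears the timer.
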(event `self.ReceiveBeginPlay`
  (bind _returnvalue (`KismetSystemLibrary.K2_SetTimerDelegate` (delegate `SpawnWaveEvent`) (`self.WaitBetweenSpawns`) true))
  (set `self.Timer` _returnvalue)
  (`self.SpawnWave`)
  (for _array_element (`self.SpawnedObstacles`)
    (`self.K2_AddActorWorldOffset` _array_element (* (`self.GetActorForwardVector` _array_element) 500.0) false false)))

(event `SpawnWaveEvent`
  (`self.SpawnWave`))

(event `self.ReceiveEndPlay`
  (params (EndPlayReason :type "EEndPlayReason Enum" :default "Destroyed"))
  (`|ExecutionSequence`
    (:`then_0`
      (for _array_element (`self.SpawnedObstacles`)
        (if (`KismetSystemLibrary.IsValid` _array_element)
          (`self.K2_DestroyActor` _array_element))))
    (:`then_1`
      (`KismetSystemLibrary.K2_ClearAndInvalidateTimerHandle` (`self.Timer`)))))

(fn `SpawnWave`
  (bind _arrow (`self.Arrow`))
  (for _index (range (`self.WaveLength`))
    (bind _returnvalue (`|SpawnActorFromClass` (`KismetArrayLibrary.Array_Random` (`self.SpawnableObstacles`)) (`KismetMathLibrary.MakeTransform` (+ (`SceneComponent.K2_GetComponentLocation` _arrow) (* _index (* -1 (`self.ObstacleOffset`)) (`SceneComponent.GetForwardVector` (`self.Arrow`)))) (`SceneComponent.K2_GetComponentRotation` _arrow) (`SceneComponent.K2_GetComponentScale` _arrow)) "Undefined" "MultiplyWithRoot" null null))
    (`KismetArrayLibrary.Array_Add` (`self.SpawnedObstacles`) _returnvalue)
    (set `/Game/BLAQ/Blueprints/PlayableArcade/Hopper/Obstacles/BP_HOPPER_Obstacle.Speed` (`self.ObstacleSpeed`) _returnvalue)
    (set `/Game/BLAQ/Blueprints/PlayableArcade/Hopper/Obstacles/BP_HOPPER_Obstacle.Spawner` self _returnvalue)))

(fn `UserConstructionScript`)