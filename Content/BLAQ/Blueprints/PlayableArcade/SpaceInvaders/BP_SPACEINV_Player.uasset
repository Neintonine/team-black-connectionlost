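; Player ship for the Space Invaders arcade minigame, moving sideways and firing shots via Enhanced Input actions.
; Movement offsets the root along world X only when a Visibility line trace finds no blocker.
; Firing spawns a shot with sound, then a timer enforces the cooldown, and overlapping an enemy shot fails the level.
; A CheckMove helper tests Y against the playfield half-width but is not called here.
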(event `self.ReceiveBeginPlay`
  (`parent.ReceiveBeginPlay`))

(event `EnhancedInput|/Game/BLAQ/Input/Actions/IA_SPACEINV_Move`
  (params (ActionValue :type "Float (double-precision)") (ElapsedSeconds :type "Float (double-precision)") (TriggeredSeconds :type "Float (double-precision)") (InputAction :type "InputAction Object Reference" :default "/Game/BLAQ/Input/Actions/IA_SPACEINV_Move.IA_SPACEINV_Move"))
  (bind _returnvalue (`SceneComponent.K2_GetComponentLocation` (`self.DefaultSceneRoot`)))
  (bind _returnvalue_2 (* ActionValue (`self.Speed`)))
  (:`Triggered`
    (bind (_outhit _returnvalue_3) (`KismetSystemLibrary.LineTraceSingle` _returnvalue (+ _returnvalue (`KismetMathLibrary.MakeVector` _returnvalue_2)) "TraceTypeQuery1"))
    (if (not _returnvalue_3)
      (`SceneComponent.K2_AddWorldOffset` (`self.DefaultSceneRoot`) (`KismetMathLibrary.MakeVector` _returnvalue_2) false false))))

(event `EnhancedInput|/Game/BLAQ/Input/Actions/IA_SPACEINV_Fire`
  (params (ActionValue :type Boolean) (ElapsedSeconds :type "Float (double-precision)") (TriggeredSeconds :type "Float (double-precision)") (InputAction :type "InputAction Object Reference" :default "/Game/BLAQ/Input/Actions/IA_SPACEINV_Fire.IA_SPACEINV_Fire"))
  (:`Triggered`
    (if (`self.IsAllowedToFire`)
      (`|SpawnActorFromClass` "/Game/BLAQ/Blueprints/PlayableArcade/SpaceInvaders/BP_SPACEINV_Shot.BP_SPACEINV_Shot_C" (`self.GetTransform`) "Undefined" "MultiplyWithRoot" self null)
      (`self.PlaySound` "/Game/BLAQ/Sound/GalaxyAttack/A_MSW_GA_Shot.A_MSW_GA_Shot")
      (set `self.IsAllowedToFire` false)
      (`KismetSystemLibrary.K2_SetTimerDelegate` (delegate `FireTrigger`) (`self.FireCooldown`)))))

(event `FireTrigger`
  (set `self.IsAllowedToFire` true))

(event `self.ReceiveActorBeginOverlap`
  (params (OtherActor :type "Actor Object Reference"))
  (if (== (`GameplayStatics.GetObjectClass` OtherActor) "/Game/BLAQ/Blueprints/PlayableArcade/SpaceInvaders/BP_SPACEINV_ShotEnemy.BP_SPACEINV_ShotEnemy_C")
    (`self.FailLevel`)))

(fn `CheckMove`
  (params (NextMove :type "Float (double-precision)"))
  (returns (Allowed :type Boolean))
  (return (< (`KismetMathLibrary.Abs` (+ NextMove (.y (`SceneComponent.K2_GetComponentLocation` (`self.DefaultSceneRoot`))))) (`self.HalfWidthPlayingField`))))

(fn `UserConstructionScript`
  (`parent.UserConstructionScript`))