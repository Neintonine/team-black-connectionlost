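; Dialogue trigger for the cash register start area, whose collision box changes state once the register reports enough tickets.
; On BeginPlay it finds the BP_CashRegister in the level, binds to its has-enough-tickets event and applies the starting collision setting to the box.
; When that event fires, the box switches to the after-paying collision setting.
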(event `self.ReceiveBeginPlay`
  (bind _returnvalue (`GameplayStatics.GetActorOfClass` "/Game/BLAQ/Assets/CashRegister/BP_CashRegister.BP_CashRegister_C"))
  (add `/Game/BLAQ/Assets/CashRegister/BP_CashRegister.HasEnoughTickets` _returnvalue (delegate `EnableCollsion`))
  (`PrimitiveComponent.SetCollisionEnabled` (`self.Box`) (`self.StartCollisionEnable`)))

(event `EnableCollsion`
  (`PrimitiveComponent.SetCollisionEnabled` (`self.Box`) (`self.AfterPayingCollision`)))

(fn `UserConstructionScript`
  (`parent.UserConstructionScript`))