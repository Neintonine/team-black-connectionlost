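; BPF_Noise is a Blueprint function set whose Noise1D function produces deterministic one-dimensional value noise from an input and a frequency.
; It seeds random streams with the truncated scaled input and the next integer to get two repeatable random values.
; An ease-in-out curve on the fractional part blends between them, and the result is remapped and clamped to the given minimum and maximum.
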(fn `Noise1D`
  (params (In :type "Float (double-precision)") (Frequency :type "Float (double-precision)" :default 1.0) (MinValue :type "Float (double-precision)") (MaxValue :type "Float (double-precision)" :default 1.0))
  (returns (ReturnValue :type "Float (double-precision)"))
  (bind _returnvalue (* In Frequency))
  (bind _returnvalue_2 (`KismetMathLibrary.FTrunc` _returnvalue))
  (bind _returnvalue_3 (`KismetMathLibrary.RandomFloatFromStream` (`KismetMathLibrary.MakeRandomStream` _returnvalue_2)))
  (return (`KismetMathLibrary.MapRangeClamped` (+ (* (`KismetMathLibrary.FInterpEaseInOut` 0.0 1.0 (`KismetMathLibrary.Fraction` _returnvalue) 2.0) (- (`KismetMathLibrary.RandomFloatFromStream` (`KismetMathLibrary.MakeRandomStream` (+ _returnvalue_2 1))) _returnvalue_3)) _returnvalue_3) 0.0 1.0 MinValue MaxValue)))