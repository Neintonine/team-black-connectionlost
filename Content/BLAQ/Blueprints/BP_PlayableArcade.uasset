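; Playable arcade cabinet that moves the first-person camera to its screen and runs a minigame from a streamed level instance.
; Interact swaps input mappings and loads the level, then a looping timer waits to hand the cabinet to BP_ArcadePlayer.
; A state enum drives the dynamic screen material, blending between start image, game render target, timed failure lockout and disabled.
; Exiting unloads the level and restores the player; completing levels awards tickets.
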(event `self.ReceiveBeginPlay`
  (`SceneComponent.SetHiddenInGame` (`self.Widget`) true false)
  (if (`self.DisableArcade`)
    (`self._ApplyState` "NewEnumerator4")))

(event `/Game/Devs/Luca/DevLevel/BPI_Interact.Interact`
  (bind _firstpersoncamera (`self.FirstPersonCamera`))
  (if (`|EnumEquality` (`self.State`) "NewEnumerator0")
    (`self.DetachPlayer`)
    (`self.LoadGame`)
    (bind (_direction _position) (`Timeline|CameraSetupAnimation` :!via `PlayFromStart`)
      (:`Update`
        (`SceneComponent.K2_SetRelativeLocationAndRotation` _firstpersoncamera (`KismetMathLibrary.VLerp` (`SceneComponent.RelativeLocation` _firstpersoncamera) (0.0 0.0 0.0) _position) (`KismetMathLibrary.RLerp` (`SceneComponent.RelativeRotation` _firstpersoncamera) (`KismetMathLibrary.MakeRotator` 0.0) _position true) false false))
      (:`Finished`
        (`SceneComponent.K2_SetWorldLocationAndRotation` (`Actor.RootComponent` (`self.FirstPersonCharacter`)) (+ (`KismetMathLibrary.MakeVector` 0.0 0.0 (`CapsuleComponent.GetScaledCapsuleHalfHeight` (`Character.CapsuleComponent` (`self.FirstPersonCharacter`)))) (`SceneComponent.K2_GetComponentLocation` (`self.PlayerExitPoint`))) (`SceneComponent.K2_GetComponentRotation` (`self.PlayerExitPoint`)) false true)))))

(event `ExitArcade`
  (params (TriggerTimeout :type Boolean))
  (bind _firstpersoncamera (`self.FirstPersonCamera`))
  (`KismetSystemLibrary.PrintText` "Exit Arcade")
  (`self.UnloadGame` TriggerTimeout)
  (`self.Reattach Player`)
  (bind (_direction _position) (`Timeline|CameraReturnTimeline` :!via `PlayFromStart`)
    (:`Update`
      (`SceneComponent.K2_SetRelativeLocationAndRotation` _firstpersoncamera (`KismetMathLibrary.VLerp` (`SceneComponent.RelativeLocation` _firstpersoncamera) (`self.FirstPersonCameraRelativePosition`) _position) (`KismetMathLibrary.RLerp` (`SceneComponent.RelativeRotation` _firstpersoncamera) (`KismetMathLibrary.MakeRotator` 0.0) _position true) false false))))

(event `MaterialGameFactorTransition`
  (params (To :type "Float (double-precision)"))
  (bind _materialparameterinfo (make `MaterialParameterInfo` "GameFactor" "BlendParameter" 0))
  (bind _returnvalue (`MaterialInstanceDynamic.K2_GetScalarParameterValueByInfo` (`self.ScreenMaterialInstance`) _materialparameterinfo))
  (bind (_direction _value) (`Timeline|GameFactorTimeline` :!via `PlayFromStart`)
    (:`Update`
      (`MaterialInstanceDynamic.SetScalarParameterValueByInfo` (`self.ScreenMaterialInstance`) _materialparameterinfo (`KismetMathLibrary.Lerp` _returnvalue To _value)))
    (:`Finished`
      (`MaterialInstanceDynamic.SetScalarParameterValueByInfo` (`self.ScreenMaterialInstance`) (make `MaterialParameterInfo` "LostFactor" "BlendParameter" 1) 0.0))))

(event `MaterialDisabledFactorTransition`
  (params (To :type "Float (double-precision)"))
  (bind _materialparameterinfo (make `MaterialParameterInfo` "LostFactor" "BlendParameter" 1))
  (bind _returnvalue (`MaterialInstanceDynamic.K2_GetScalarParameterValueByInfo` (`self.ScreenMaterialInstance`) _materialparameterinfo))
  (bind (_direction _value) (`Timeline|DisabledFactorTimeline` :!via `PlayFromStart`)
    (:`Update`
      (`MaterialInstanceDynamic.SetScalarParameterValueByInfo` (`self.ScreenMaterialInstance`) _materialparameterinfo (`KismetMathLibrary.Lerp` _returnvalue To _value)))))

(event `self.ReceiveTick`
  (params (DeltaSeconds :type "Float (single-precision)"))
  (if (`KismetSystemLibrary.K2_IsTimerActiveHandle` (`self.TimeoutTimer`))
    (`MaterialInstanceDynamic.SetScalarParameterValueByInfo` (`self.ScreenMaterialInstance`) (make `MaterialParameterInfo` "TimerElapsed" "LayerParameter" 2) (/ (`KismetSystemLibrary.K2_GetTimerElapsedTimeHandle` (`self.TimeoutTimer`)) (`self.TimeoutDuration`)))))

(event `self.Box.OnComponentBeginOverlap`
  (params (OverlappedComponent :type "PrimitiveComponent Object Reference") (OtherActor :type "Actor Object Reference") (OtherComp :type "PrimitiveComponent Object Reference") (OtherBodyIndex :type Integer) (bFromSweep :type Boolean) (SweepResult :type "HitResult Structure (by ref)"))
  (if (`|EnumEquality` (`self.State`) "NewEnumerator0")
    (cast `/Game/FirstPerson/Blueprints/BP_FirstPersonCharacter` OtherActor)
    (`SceneComponent.SetHiddenInGame` (`self.Widget`) false false)))

(event `self.Box.OnComponentEndOverlap`
  (params (OverlappedComponent :type "PrimitiveComponent Object Reference") (OtherActor :type "Actor Object Reference") (OtherComp :type "PrimitiveComponent Object Reference") (OtherBodyIndex :type Integer))
  (if (`|EnumEquality` (`self.State`) "NewEnumerator0")
    (cast `/Game/FirstPerson/Blueprints/BP_FirstPersonCharacter` OtherActor)
    (`SceneComponent.SetHiddenInGame` (`self.Widget`) true false)))

(fn `_ApplyState`
  (params (State :type "/Game/BLAQ/Blueprints/E_ArcadeMachineState Enum" :default "NewEnumerator0"))
  (bind _materialparameterinfo (make `MaterialParameterInfo` "GameTexture" "LayerParameter" 1))
  (bind _gameviewrendertarget (`self.GameViewRenderTarget`))
  (bind _screenmaterialinstance (`self.ScreenMaterialInstance`))
  (bind _output_get (set `self.State` State))
  (switch `/Game/BLAQ/Blueprints/E_ArcadeMachineState` _output_get
    (:`NewEnumerator0`
      (`self.MaterialGameFactorTransition` 0.0 :!label _label))
    (:`NewEnumerator3`
      (goto _label))
    (:`NewEnumerator1`
      (`MaterialInstanceDynamic.SetTextureParameterValueByInfo` _screenmaterialinstance _materialparameterinfo _gameviewrendertarget)
      (`self.MaterialGameFactorTransition` 1.0))
    (:`NewEnumerator2`
      (`MaterialInstanceDynamic.SetTextureParameterValueByInfo` _screenmaterialinstance _materialparameterinfo _gameviewrendertarget)
      (`self.MaterialDisabledFactorTransition` 1.0))
    (:`NewEnumerator4`
      (`MaterialInstanceDynamic.SetScalarParameterValueByInfo` (`self.ScreenMaterialInstance`) (make `MaterialParameterInfo` "DisabledFactor" "BlendParameter" 2) 1.0))))

(fn `_UndoTimeout`
  (`self._ApplyState` "NewEnumerator0"))

(fn `AttachArcadeToGame`
  (if (`LevelStreaming.IsLevelLoaded` (`self.LoadedLevel`))
    (bind _returnvalue (`GameplayStatics.GetActorOfClass` "/Game/BLAQ/Blueprints/BP_ArcadePlayer.BP_ArcadePlayer_C"))
    (if (`KismetSystemLibrary.IsValid` _returnvalue)
      (`KismetSystemLibrary.K2_ClearAndInvalidateTimerHandle` (`self.AttachTimer`))
      (`/Game/BLAQ/Blueprints/BP_ArcadePlayer.Setup` _returnvalue self)
      (`self._ApplyState` "NewEnumerator1"))))

(fn `CompleteLevel`
  (set `self.CurrentLevel` (+ (`self.CurrentLevel`) 1))
  (`/Game/FirstPerson/Blueprints/BP_FirstPersonCharacter.Add Tickets` (`self.FirstPersonCharacter`) (`self.TicketRewardPerLevel`)))

(fn `DetachPlayer`
  (`SceneComponent.SetHiddenInGame` (`self.Widget`) true false)
  (`EnhancedInputSubsystemInterface.ClearAllMappings` (pcsubsystem `EnhancedInputLocalPlayerSubsystem` (`GameplayStatics.GetPlayerController` 0)))
  (bind _asbp_first_person_character (cast `/Game/FirstPerson/Blueprints/BP_FirstPersonCharacter` (`GameplayStatics.GetPlayerCharacter` 0)))
  (set `self.FirstPersonCharacter` _asbp_first_person_character)
  (bind _firstpersoncamera (`/Game/FirstPerson/Blueprints/BP_FirstPersonCharacter.FirstPersonCamera` _asbp_first_person_character))
  (set `self.FirstPersonCameraRelativePosition` (`SceneComponent.RelativeLocation` _firstpersoncamera))
  (set `self.FirstPersonCameraRelativeRotation` (`SceneComponent.RelativeRotation` _firstpersoncamera))
  (bind _output_get (set `self.FirstPersonCamera` _firstpersoncamera))
  (`SceneComponent.K2_AttachToComponent` _output_get (`self.CameraTarget`) "None" "KeepWorld" "KeepWorld" "KeepWorld" true))

(fn `GetFirstPersonController`
  (returns (FirstPersonCamera :type "CameraComponent Object Reference"))
  (return (`self.FirstPersonCamera`)))

(fn `LoadGame`
  (`EnhancedInputSubsystemInterface.AddMappingContext` (pcsubsystem `EnhancedInputLocalPlayerSubsystem` (`GameplayStatics.GetPlayerController` 0)) "/Game/BLAQ/Input/IMC_Arcade.IMC_Arcade" 0 (struct))
  (bind (_boutsuccess _returnvalue) (`LevelStreamingDynamic.LoadLevelInstanceBySoftObjectPtr` (`self.Level`) (0.0 5000.0 0.0) (struct) "" null))
  (if _boutsuccess
    (set `self.LoadedLevel` _returnvalue)
    (bind _returnvalue_2 (`KismetSystemLibrary.K2_SetTimer` null "AttachArcadeToGame" 0.05 true))
    (set `self.AttachTimer` _returnvalue_2)
    (`self._ApplyState` "NewEnumerator3")
    (else
      (`KismetSystemLibrary.PrintText` "Couldn't load Minigame"))))

(fn `Reattach Player`
  (bind _returnvalue (`GameplayStatics.GetPlayerController` 0))
  (bind _returnvalue_2 (pcsubsystem `EnhancedInputLocalPlayerSubsystem` _returnvalue))
  (`EnhancedInputSubsystemInterface.ClearAllMappings` _returnvalue_2)
  (`EnhancedInputSubsystemInterface.AddMappingContext` _returnvalue_2 "/Game/FirstPerson/Input/IMC_Default.IMC_Default" 0 (struct))
  (`Controller.Possess` _returnvalue (`self.FirstPersonCharacter`))
  (`SceneComponent.K2_AttachToComponent` (`self.FirstPersonCamera`) (`Character.CapsuleComponent` (`self.FirstPersonCharacter`)) "None" "KeepWorld" "KeepWorld" "KeepWorld" true))

(fn `TriggerTimeout`
  (bind _returnvalue (`KismetSystemLibrary.K2_SetTimer` null "_UndoTimeout" (`self.TimeoutDuration`)))
  (set `self.TimeoutTimer` _returnvalue)
  (`self._ApplyState` "NewEnumerator2"))

(fn `UnloadGame`
  (params (TriggerTimeout :type Boolean))
  (set `LevelStreaming.bShouldBeLoaded` false (`self.LoadedLevel`))
  (if TriggerTimeout
    (`self.TriggerTimeout`)
    (else
      (`self._ApplyState` "NewEnumerator0"))))

(fn `UserConstructionScript`
  (bind _returnvalue (`PrimitiveComponent.CreateDynamicMaterialInstance` (`self.Mesh`) (`self.ScreenMaterialIndex`) "/Game/BLAQ/Materials/Screen/PlayableArcade/M_PlayableArcade_Screen.M_PlayableArcade_Screen" "None"))
  (bind _output_get (set `self.ScreenMaterialInstance` _returnvalue))
  (`MaterialInstanceDynamic.SetTextureParameterValueByInfo` _output_get (make `MaterialParameterInfo` "StartImage" "LayerParameter" 0) (`self.StartTexture`)))