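; BP_Safezone is an actor that shelters the first-person player from the enemy AI monster.
; One tick after BeginPlay it caches a single BP_EnemyAI found with GetActorOfClass.
; When the player character begins overlapping, it cancels that monster's chase and disables its sensing of the player.
; When the player leaves, it re-enables sensing without restarting the chase.
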(event `self.ReceiveBeginPlay`
  (`KismetSystemLibrary.DelayUntilNextTick`)
  (bind _returnvalue (`GameplayStatics.GetActorOfClass` "/Game/BLAQ/Assets/Monster/BP_EnemyAI.BP_EnemyAI_C"))
  (set `self.Monster` _returnvalue))

(event `self.ReceiveActorBeginOverlap`
  (params (OtherActor :type "Actor Object Reference"))
  (cast `/Game/FirstPerson/Blueprints/BP_FirstPersonCharacter` OtherActor)
  (`/Game/BLAQ/Assets/Monster/BP_EnemyAI.SetChase` (`self.Monster`) false)
  (set `/Game/BLAQ/Assets/Monster/BP_EnemyAI.AllowSensingPlayer` false (`self.Monster`)))

(event `self.ReceiveActorEndOverlap`
  (params (OtherActor :type "Actor Object Reference"))
  (cast `/Game/FirstPerson/Blueprints/BP_FirstPersonCharacter` OtherActor)
  (set `/Game/BLAQ/Assets/Monster/BP_EnemyAI.AllowSensingPlayer` true (`self.Monster`)))

(fn `UserConstructionScript`)