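; CCTV monitor actor that shows the live scene capture of a linked camera on its screen.
; On BeginPlay, if the first linked camera is valid, it creates a render target sized from aspect ratio and pixel resolution and assigns it to that camera's SceneCaptureComponent2D.
; A dynamic M_CCTV material on the monitor mesh's screen slot displays that target.
; Only the first entry in LinkedCameras is used.
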(event `self.ReceiveBeginPlay`
  (bind (_returnvalue_x _returnvalue_y) (`KismetMathLibrary.BreakVector2D` (* (`self.AspectRatio`) (`self.ScreenResInPixel`))))
  (`/Engine/EditorBlueprintResources/StandardMacros.IsValid` (`|GetArrayItem` (`self.LinkedCameras`))
    (:`Is Valid`
      (bind _returnvalue (`KismetMaterialLibrary.CreateDynamicMaterialInstance` "/Game/BLAQ/Assets/Monitor/M_CCTV.M_CCTV"))
      (bind _output_get (set `self.M_Screen` _returnvalue))
      (`PrimitiveComponent.SetMaterial` (`self.SM_monitor_01_a`) 1 _output_get)
      (bind _returnvalue_2 (`KismetRenderingLibrary.CreateRenderTarget2D` (`KismetMathLibrary.FTrunc` _returnvalue_x) (`KismetMathLibrary.FTrunc` _returnvalue_y)))
      (bind _output_get_2 (set `self.CCTV_RT` _returnvalue_2))
      (bind _output_get_3 (set `SceneCaptureComponent2D.TextureTarget` _output_get_2 (`/Game/BLAQ/Blueprints/BP_CCTV.SceneCaptureComponent2D` (`|GetArrayItem` (`self.LinkedCameras`)))))
      (`MaterialInstanceDynamic.SetTextureParameterValue` (`self.M_Screen`) "CCTV" _output_get_3))))

(fn `UserConstructionScript`)