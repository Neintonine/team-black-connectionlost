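; BP_SPACEINV_Shot is a projectile actor for the Space Invaders game.
; Each tick it moves its root along the world Y axis, scaled by MoveDirection, MoveSpeed and delta time, so the direction variable sets which way it travels.
; On overlap it destroys itself unless the other actor's exact class is in the IgnoreClasses list.
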(event `self.ReceiveTick`
  (params (DeltaSeconds :type "Float (single-precision)"))
  (if true
    (`SceneComponent.K2_AddWorldOffset` (`self.DefaultSceneRoot`) (`KismetMathLibrary.MakeVector` 0.0 (* DeltaSeconds (`self.MoveDirection`) (`self.MoveSpeed`))) false false)))

(event `self.ReceiveActorBeginOverlap`
  (params (OtherActor :type "Actor Object Reference"))
  (if (not (`KismetArrayLibrary.Array_Contains` (`self.IgnoreClasses`) (`GameplayStatics.GetObjectClass` OtherActor)))
    (`self.K2_DestroyActor`)))

(fn `UserConstructionScript`)