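; Space Invaders alien spawner that builds and drives the enemy formation and decides level completion or failure.
; Spawn fills random grid cells with attached aliens, meshed by row, and shortens the move interval as Level rises.
; Ticker checks step aliens sideways, periodically shift the root along Y, failing the player if aliens get too close, and separately fire shots from random aliens.
; InformAlienDeath removes dead aliens and completes the level when none remain.
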(event `self.ReceiveBeginPlay`
  (set `self.StartPosition` (`SceneComponent.K2_GetComponentLocation` (`self.DefaultSceneRoot`))))

(event `self.ReceiveTick`
  (params (DeltaSeconds :type "Float (single-precision)"))
  (bind (_returnvalue_x _returnvalue_y) (`KismetMathLibrary.BreakVector` (`SceneComponent.K2_GetComponentLocation` (`/Game/BLAQ/Blueprints/BP_ArcadePlayer.DefaultSceneRoot` (`self.Player`)))))
  (`|ExecutionSequence`
    (:`then_0`
      (bind _allowed (`/Game/BLAQ/Blueprints/BP_ArcadeTicker.CheckTick` (`self.Ticker`) (`self.MoveTickDifference`) 0))
      (if _allowed
        (bind _output_get (set `self.AlienCurrentSteps` (+ (`self.AlienCurrentSteps`) 1)))
        (if (>= _output_get (`self.AlienMaxSteps`))
          (set `self.AlienCurrentSteps` 0)
          (for _array_element (`self.SpawnedAliens`)
            (`/Engine/EditorBlueprintResources/StandardMacros.IsValid` _array_element
              (:`Is Valid`
                (set `/Game/BLAQ/Blueprints/SpaceInvaders/BP_SPACEINV_Alien.RowIndex` (+ (`/Game/BLAQ/Blueprints/SpaceInvaders/BP_SPACEINV_Alien.RowIndex` _array_element) 1) _array_element))))
          (`SceneComponent.K2_AddWorldOffset` (`self.DefaultSceneRoot`) (`KismetMathLibrary.MakeVector` 0.0 (`/Game/BLAQ/Blueprints/BP_Arcade_Definitions.GetGridSize`)) false false)
          (for _array_element_2 (`self.SpawnedAliens`)
            (`/Engine/EditorBlueprintResources/StandardMacros.IsValid` _array_element_2
              (:`Is Valid`
                (bind (_returnvalue_x_2 _returnvalue_y_2) (`KismetMathLibrary.BreakVector` (`SceneComponent.K2_GetComponentLocation` (`/Game/BLAQ/Blueprints/SpaceInvaders/BP_SPACEINV_Alien.DefaultSceneRoot` _array_element_2))))
                (if (<= (`KismetMathLibrary.Abs` (- _returnvalue_y_2 _returnvalue_y)) (`self.MinYPosition`))
                  (`/Game/BLAQ/Blueprints/BP_ArcadePlayer.FailLevel` (`self.Player`))
                  (break)))))
          (else
            (for _array_element_3 (`self.SpawnedAliens`)
              (`/Game/BLAQ/Blueprints/SpaceInvaders/BP_SPACEINV_Alien.MoveHorizontal` _array_element_3))))))
    (:`then_1`
      (bind _allowed_2 (`/Game/BLAQ/Blueprints/BP_ArcadeTicker.CheckTick` (`self.Ticker`) 10 1))
      (if _allowed_2
        (`|SpawnActorFromClass` "/Game/BLAQ/Blueprints/SpaceInvaders/BP_SPACEINV_ShotEnemy.BP_SPACEINV_ShotEnemy_C" (`self.GetTransform` (`|GetArrayItem` (`self.SpawnedAliens`) (`KismetMathLibrary.RandomInteger` (`KismetArrayLibrary.Array_Length` (`self.SpawnedAliens`))))) "Undefined" "MultiplyWithRoot" self null)))))

(fn `_CalculateAlienPosition`
  (params (`X Index` :type Integer) (`Y Index` :type Integer))
  (returns (Position :type "Vector Structure"))
  (bind _aliengrid_x (`KismetMathLibrary.BreakVector2D` (`self.AlienGrid`)))
  (return (+ (`KismetMathLibrary.MakeVector` (* (- `X Index` (/ _aliengrid_x 2) -0.5) (`/Game/BLAQ/Blueprints/BP_Arcade_Definitions.GetGridSize`) 3.0) (* `Y Index` (`/Game/BLAQ/Blueprints/BP_Arcade_Definitions.GetGridSize`) 4.0)) (`SceneComponent.K2_GetComponentLocation` (`self.DefaultSceneRoot`)))))

(fn `InformAlienDeath`
  (params (Alien :type "/Game/BLAQ/Blueprints/SpaceInvaders/BP_SPACEINV_Alien Object Reference"))
  (`/Game/BLAQ/Blueprints/BP_ArcadePlayer.PlaySound` (`self.Player`) "/Game/Devs/Michel/Sounds/GalaxyAttack/A_GA_AlienDeath.A_GA_AlienDeath")
  (`KismetArrayLibrary.Array_RemoveItem` (`self.SpawnedAliens`) Alien)
  (if (< (`KismetArrayLibrary.Array_Length` (`self.SpawnedAliens`)) 1)
    (`/Game/BLAQ/Blueprints/BP_ArcadePlayer.CompleteLevel` (`self.Player`))))

(fn `Spawn`
  (params (Level :type Integer) (Reason :type "/Game/BLAQ/Blueprints/BPE_ArcadeSpawnReason Enum" :default "NewEnumerator0"))
  (locals (PossibleSpawnLocations :type "Array of Vector2D Structure"))
  (bind _alienrange (`self.AlienRange`))
  (bind _aliengrid_x (`KismetMathLibrary.BreakVector2D` (`self.AlienGrid`)))
  (bind (_aliengrid_x_2 _aliengrid_y) (`KismetMathLibrary.BreakVector2D` (`self.AlienGrid`)))
  (bind _movetickrange (`self.MoveTickRange`))
  (bind (_outitem _outindex) (`KismetArrayLibrary.Array_Random` (`local.PossibleSpawnLocations`)))
  (bind _returnvalue (`KismetMathLibrary.FTrunc` (`.Y` (`KismetMathLibrary.BreakVector2D` _outitem))))
  (`SceneComponent.K2_SetWorldLocation` (`self.DefaultSceneRoot`) (`self.StartPosition`) false false)
  (set `self.MoveTickDifference` (`KismetMathLibrary.Max` (`.Value` (break `Int32RangeBound` (break `Int32Range` _movetickrange))) (- (`.Value` (break `Int32RangeBound` (`.UpperBound` (break `Int32Range` _movetickrange)))) (/ (+ Level 1) 2))))
  (set `self.AlienCurrentSteps` (/ (`self.AlienMaxSteps`) 2))
  (for _index (range (+ (`KismetMathLibrary.FTrunc` (- _aliengrid_y 1.0)) 1))
    (for _index_2 (range (+ (`KismetMathLibrary.FTrunc` (- _aliengrid_x 1.0)) 1))
      (`KismetArrayLibrary.Array_Add` (`local.PossibleSpawnLocations`) (`KismetMathLibrary.MakeVector2D` (`KismetMathLibrary.Conv_IntToDouble` _index_2) (`KismetMathLibrary.Conv_IntToDouble` _index)))))
  (for _ (range (`KismetMathLibrary.Min` (+ (* 0 (`self.AliensPerLevel`)) (`.Value` (break `Int32RangeBound` (break `Int32Range` _alienrange)))) (`.Value` (break `Int32RangeBound` (`.UpperBound` (break `Int32Range` _alienrange))))))
    (bind _returnvalue_2 (`|SpawnActorFromClass` "/Game/BLAQ/Blueprints/SpaceInvaders/BP_SPACEINV_Alien.BP_SPACEINV_Alien_C" (`KismetMathLibrary.MakeTransform` (`self._CalculateAlienPosition` (`KismetMathLibrary.FTrunc` (`KismetMathLibrary.BreakVector2D` _outitem)) _returnvalue)) "Undefined" "MultiplyWithRoot" self null))
    (`StaticMeshComponent.SetStaticMesh` (`/Game/BLAQ/Blueprints/SpaceInvaders/BP_SPACEINV_Alien.Mesh` _returnvalue_2) (`|GetArrayItem` (`self.Meshes`) _returnvalue))
    (set `/Game/BLAQ/Blueprints/SpaceInvaders/BP_SPACEINV_Alien.RowIndex` _returnvalue _returnvalue_2)
    (set `/Game/BLAQ/Blueprints/SpaceInvaders/BP_SPACEINV_Alien.Spawner` self _returnvalue_2)
    (`KismetArrayLibrary.Array_Add` (`self.SpawnedAliens`) _returnvalue_2)
    (`KismetArrayLibrary.Array_Remove` (`local.PossibleSpawnLocations`) _outindex)
    (`self.K2_AttachToActor` _returnvalue_2 self "None" "KeepWorld" "KeepWorld" "KeepWorld" true)))

(fn `UserConstructionScript`)