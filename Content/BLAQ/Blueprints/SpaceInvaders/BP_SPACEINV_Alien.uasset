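; Alien enemy for a Space Invaders game that dies when hit by a shot.
; Overlapping a BP_SPACEINV_Shot actor destroys the alien and reports its death to its Spawner.
; MoveHorizontal offsets it along world X by a fraction of the grid size, with row index parity setting the direction so alternate rows move opposite ways.
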(event `self.ReceiveActorBeginOverlap`
  (params (OtherActor :type "Actor Object Reference"))
  (if (== "/Game/BLAQ/Blueprints/SpaceInvaders/BP_SPACEINV_Shot.BP_SPACEINV_Shot_C" (`GameplayStatics.GetObjectClass` OtherActor))
    (`self.K2_DestroyActor`)
    (`/Game/BLAQ/Blueprints/SpaceInvaders/BP_SPACEINV_AlienSpawner.InformAlienDeath` (`self.Spawner`) self)))

(fn `MoveHorizontal`
  (`SceneComponent.K2_AddWorldOffset` (`self.DefaultSceneRoot`) (`KismetMathLibrary.MakeVector` (* (`/Game/BLAQ/Blueprints/BP_Arcade_Definitions.GetGridSize`) (`KismetMathLibrary.SelectFloat` -1.0 1.0 (> (mod (`KismetMathLibrary.Conv_IntToDouble` (`self.RowIndex`)) 2.0) 0.0)) 0.75)) false false))

(fn `UserConstructionScript`)