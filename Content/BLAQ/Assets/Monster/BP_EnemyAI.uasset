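; Enemy monster pawn that detects the player and dims arcade lights as it moves through the level.
; Its PawnSensing component sets the "HasSeenPlayer?" blackboard flag on its AI controller when it sees the first-person character; nothing here clears it.
; Overlapping a BP_Arcade actor dims that arcade's lights, and ending the overlap brightens them again.
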(event `self.ReceiveActorEndOverlap`
  (params (OtherActor :type "Actor Object Reference"))
  (bind _asbp_arcade (cast `/Game/BLAQ/Assets/Arcade-Machine/BP_Arcade` OtherActor))
  (`/Game/BLAQ/Assets/Arcade-Machine/BP_Arcade.BrightenLights` _asbp_arcade))

(event `self.ReceiveActorBeginOverlap`
  (params (OtherActor :type "Actor Object Reference"))
  (bind _asbp_arcade (cast `/Game/BLAQ/Assets/Arcade-Machine/BP_Arcade` OtherActor))
  (`/Game/BLAQ/Assets/Arcade-Machine/BP_Arcade.DimLights` _asbp_arcade))

(event `self.PawnSensing.OnSeePawn`
  (params (Pawn :type "Pawn Object Reference"))
  (cast `/Game/FirstPerson/Blueprints/BP_FirstPersonCharacter` Pawn)
  (`BlackboardComponent.SetValueAsBool` (`AIBlueprintHelperLibrary.GetBlackboard` (`AIBlueprintHelperLibrary.GetAIController` self)) "HasSeenPlayer?" true))

(fn `UserConstructionScript`)