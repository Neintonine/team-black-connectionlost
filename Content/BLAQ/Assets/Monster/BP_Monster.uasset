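; BP_Monster is a monster actor that repeatedly travels along a fixed line and affects arcade lighting as it passes.
; Each Tick lowers its root's X by LocationOffset, without delta-time scaling, then teleports it back to the start beyond a threshold.
; The Delay after the reset has nothing following it, so it does not pause movement.
; Overlapping a BP_Arcade calls DimLights, and ending the overlap calls BrightenLights.
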(event `self.ReceiveTick`
  (params (DeltaSeconds :type "Float (single-precision)"))
  (bind _defaultsceneroot (`self.DefaultSceneRoot`))
  (bind _returnvalue_x (`KismetMathLibrary.BreakVector` (`SceneComponent.K2_GetComponentLocation` _defaultsceneroot)))
  (if (> _returnvalue_x -1200.0)
    (`SceneComponent.K2_SetWorldLocation` (`self.DefaultSceneRoot`) (`KismetMathLibrary.MakeVector` (- _returnvalue_x (`self.Location Offset`)) 25.0 -5.0) false false)
    (else
      (`SceneComponent.K2_SetWorldLocation` _defaultsceneroot (929.186715 25.0 -5.0) false false)
      (`KismetSystemLibrary.Delay` 10.0))))

(event `self.ReceiveActorBeginOverlap`
  (params (OtherActor :type "Actor Object Reference"))
  (bind _asbp_arcade (cast `/Game/BLAQ/Assets/Arcade-Machine/BP_Arcade` OtherActor)
    (:`then`
      (`/Game/BLAQ/Assets/Arcade-Machine/BP_Arcade.DimLights` _asbp_arcade))
    (:`CastFailed`
      (`KismetSystemLibrary.PrintString` "shit"))))

(event `self.ReceiveActorEndOverlap`
  (params (OtherActor :type "Actor Object Reference"))
  (bind _asbp_arcade (cast `/Game/BLAQ/Assets/Arcade-Machine/BP_Arcade` OtherActor))
  (`/Game/BLAQ/Assets/Arcade-Machine/BP_Arcade.BrightenLights` _asbp_arcade))

(fn `UserConstructionScript`)