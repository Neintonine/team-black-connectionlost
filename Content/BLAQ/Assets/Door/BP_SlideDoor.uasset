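; Sliding double door that opens when the cash register signals that the player has enough tickets.
; Binds to BP_CashRegister on BeginPlay; the event plays audio and runs a timeline that slides two arrow components apart by DoorDistance.
; Ending an actor overlap reverses the timeline to close it.
; The construction script places both arrows at their open offsets, BeginPlay resets them to closed, and the Open function is an empty stub.
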(event `self.ReceiveBeginPlay`
  (`|ExecutionSequence`
    (:`then_0`
      (`SceneComponent.K2_SetRelativeLocation` (`self.Arrow1`) (0.0 0.0 0.0) false false)
      (`SceneComponent.K2_SetRelativeLocation` (`self.Arrow`) (0.0 0.0 0.0) false false))
    (:`then_1`
      (bind _returnvalue (`GameplayStatics.GetActorOfClass` "/Game/BLAQ/Assets/CashRegister/BP_CashRegister.BP_CashRegister_C"))
      (add `/Game/BLAQ/Assets/CashRegister/BP_CashRegister.HasEnoughTickets` _returnvalue (delegate `DoorOpener`)))))

(event `DoorOpener`
  (`AudioComponent.Play` (`self.Audio`) 0.0)
  (bind (_direction _dooropen) (`Timeline|Timeline` :!label _label)
    (:`Update`
      (`|ExecutionSequence`
        (:`then_0`
          (bind _returnvalue (* _dooropen (`self.DoorDistance`)))
          (`SceneComponent.K2_SetRelativeLocation` (`self.Arrow1`) (`KismetMathLibrary.MakeVector` _returnvalue) false false))
        (:`then_1`
          (`SceneComponent.K2_SetRelativeLocation` (`self.Arrow`) (`KismetMathLibrary.MakeVector` (* _returnvalue -1.0)) false false))))))

(event `self.ReceiveActorEndOverlap`
  (params (OtherActor :type "Actor Object Reference"))
  (goto _label :!via `Reverse`))

(fn `Open`)

(fn `UserConstructionScript`
  (bind _doordistance (`self.DoorDistance`))
  (`|ExecutionSequence`
    (:`then_0`
      (`SceneComponent.K2_SetRelativeLocation` (`self.Arrow1`) (`KismetMathLibrary.MakeVector` _doordistance) false false))
    (:`then_1`
      (`SceneComponent.K2_SetRelativeLocation` (`self.Arrow`) (`KismetMathLibrary.MakeVector` (* _doordistance -1.0)) false false))))