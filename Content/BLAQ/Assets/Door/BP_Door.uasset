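; BP_Door is a door actor that opens when the player character overlaps it and closes when they leave.
; Begin overlap plays a timeline and end overlap reverses it, with both filtered to player character 0.
; The timeline's OpenDoorTIme track sets the relative yaw of an Arrow component, which appears to act as the hinge.
; Opening also prints a "Door Open" debug message.
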(event `self.ReceiveActorBeginOverlap`
  (params (OtherActor :type "Actor Object Reference"))
  (if (== OtherActor (`GameplayStatics.GetPlayerCharacter` 0))
    (`KismetSystemLibrary.PrintString` "Door Open")
    ;[1 1 1] Opens the door over Time
    (bind (_direction _open_door_time) (`Timeline|Timeline` :!label _label)
      (:`Update`
        (`SceneComponent.K2_SetRelativeRotation` (`self.Arrow`) (`KismetMathLibrary.MakeRotator` 0.0 0.0 _open_door_time) false false)))))

(event `self.ReceiveActorEndOverlap`
  (params (OtherActor :type "Actor Object Reference"))
  (if (== OtherActor (`GameplayStatics.GetPlayerCharacter` 0))
    (goto _label :!via `Reverse`)))

(fn `UserConstructionScript`)