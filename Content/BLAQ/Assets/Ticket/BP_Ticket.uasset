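; BP_Ticket is a collectible pickup that awards tickets to the player.
; Every tick, Bogging moves and spins the Arrow component by adding a sine-based local offset and a yaw delta scaled by elapsed time.
; On player overlap, it detaches the ticket mesh and a timeline lerps it toward the character's mesh.
; When the timeline finishes, it adds Value to BP_FirstPersonCharacter's tickets and destroys itself.
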(event `self.ReceiveActorBeginOverlap`
  (params (OtherActor :type "Actor Object Reference"))
  (if (== OtherActor (`GameplayStatics.GetPlayerCharacter` 0))
    (`SceneComponent.K2_DetachFromComponent` (`self.SM_Ticket`) "KeepWorld" "KeepWorld" "KeepWorld" true)
    (bind (_direction _newtrack_1) (`Timeline|Timeline`)
      (:`Update`
        (`SceneComponent.K2_SetWorldLocation` (`self.SM_Ticket`) (`KismetMathLibrary.VLerp` (`SceneComponent.K2_GetComponentLocation` (`self.SM_Ticket`)) (`SceneComponent.K2_GetComponentLocation` (`Character.Mesh` (`GameplayStatics.GetPlayerCharacter` 0))) _newtrack_1) false false))
      (:`Finished`
        (bind _asbp_first_person_character (cast `/Game/FirstPerson/Blueprints/BP_FirstPersonCharacter` OtherActor))
        (`/Game/FirstPerson/Blueprints/BP_FirstPersonCharacter.Add Tickets` _asbp_first_person_character (`self.Value`))
        (`self.K2_DestroyActor`)))))

(event `self.ReceiveTick`
  (params (DeltaSeconds :type "Float (single-precision)"))
  (`self.Bogging`))

(event `self.ReceiveBeginPlay`
  ;[1 1 1] Store original location to center around for bobbing
  (set `self.TicketStartLocation` (`SceneComponent.RelativeLocation` (`self.Arrow`))))

(fn `UserConstructionScript`)