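; BP_TicketChangeLevel is a collectible ticket pickup that bobs and spins through its Arrow component on Tick.
; Sphere overlaps with the first-person character show or hide a Widget.
; Interact checks the overlapped actor is the player, then a Timeline pulls the detached ticket mesh toward the player's mesh.
; When finished, it adds Value to the player's tickets, displays inner dialogue and destroys itself; no level-change logic is present.
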(event `self.Interact`
  (if (== (`GameplayStatics.GetPlayerCharacter` 0) (stale `self.Sphere.OnComponentBeginOverlap` OtherActor))
    (`SceneComponent.K2_DetachFromComponent` (`self.SM_Ticket`) "KeepWorld" "KeepWorld" "KeepWorld" true)
    (bind (_direction _newtrack_1) (`Timeline|Timeline`)
      (:`Update`
        (`SceneComponent.K2_SetWorldLocation` (`self.SM_Ticket`) (`KismetMathLibrary.VLerp` (`SceneComponent.K2_GetComponentLocation` (`self.SM_Ticket`)) (`SceneComponent.K2_GetComponentLocation` (`Character.Mesh` (`GameplayStatics.GetPlayerCharacter` 0))) _newtrack_1) false false))
      (:`Finished`
        (bind _asbp_first_person_character (cast `/Game/FirstPerson/Blueprints/BP_FirstPersonCharacter` (`GameplayStatics.GetPlayerCharacter` 0)))
        (`/Game/FirstPerson/Blueprints/BP_FirstPersonCharacter.Add Tickets` _asbp_first_person_character (`self.Value`))
        (`/Game/BLAQ/Blueprints/Dialouge/BP_UI_Dialogue.DisplayInnerDialogue` (`/Game/FirstPerson/Blueprints/BP_FirstPersonCharacter.Dialogue` _asbp_first_person_character) "Oh good, a forgotten ticket. No playing on these dumb machines.")
        (`self.K2_DestroyActor`)))))

(event `self.Sphere.OnComponentBeginOverlap`
  (params (OverlappedComponent :type "PrimitiveComponent Object Reference") (OtherActor :type "Actor Object Reference") (OtherComp :type "PrimitiveComponent Object Reference") (OtherBodyIndex :type Integer) (bFromSweep :type Boolean) (SweepResult :type "HitResult Structure (by ref)"))
  (cast `/Game/FirstPerson/Blueprints/BP_FirstPersonCharacter` OtherActor)
  (`SceneComponent.SetHiddenInGame` (`self.Widget`) false false))

(event `self.Sphere.OnComponentEndOverlap`
  (params (OverlappedComponent :type "PrimitiveComponent Object Reference") (OtherActor :type "Actor Object Reference") (OtherComp :type "PrimitiveComponent Object Reference") (OtherBodyIndex :type Integer))
  (cast `/Game/FirstPerson/Blueprints/BP_FirstPersonCharacter` OtherActor)
  (`SceneComponent.SetHiddenInGame` (`self.Widget`) true false))

(event `self.ReceiveTick`
  (params (DeltaSeconds :type "Float (single-precision)"))
  (`self.Bogging` DeltaSeconds))

(event `self.ReceiveBeginPlay`
  ;[1 1 1] Store original location to center around for bobbing
  (set `self.TicketStartLocation` (`SceneComponent.RelativeLocation` (`self.Arrow`))))

(fn `UserConstructionScript`)