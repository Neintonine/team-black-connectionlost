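; Arcade machine prop actor that varies its cabinet and screen and reacts to lighting events.
; The construction script picks one of four arcade meshes at random.
; BeginPlay and BrightenLights assign a random glowing or flickering screen material to the first material slot.
; DimLights briefly turns the screen red, then switches it to a black background after a short delay.
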(event `self.ReceiveBeginPlay`
  (bind _sm_arcade_2 (`self.SM_Arcade-2`))
  (`|ExecutionSequence`
    (:`then_1`
      ;[1 1 1] Random Screen Material
      (switch `int` (`KismetMathLibrary.RandomIntegerInRange` 0 2) :!label _label
        (:`0`
          (`PrimitiveComponent.SetMaterial` _sm_arcade_2 0 "/Game/BLAQ/Assets/Arcade-Machine/MI_ScreenGlowing.MI_ScreenGlowing"))
        (:`1`
          (`PrimitiveComponent.SetMaterial` _sm_arcade_2 0 "/Game/BLAQ/Assets/Arcade-Machine/MI_ScreenGlowing1.MI_ScreenGlowing1"))
        (:`2`
          (`PrimitiveComponent.SetMaterial` _sm_arcade_2 0 "/Game/BLAQ/Assets/Arcade-Machine/M_FlickeringGlow.M_FlickeringGlow"))))))

(event `BrightenLights`
  (goto _label))

(event `DimLights`
  (`PrimitiveComponent.SetMaterial` (`self.SM_Arcade-2`) 0 "/Game/BLAQ/Assets/Arcade-Machine/MI_ScreenRed.MI_ScreenRed")
  (`KismetSystemLibrary.Delay` 0.2)
  (`PrimitiveComponent.SetMaterial` (`self.SM_Arcade-2`) 0 "/Engine/MapTemplates/Sky/M_BlackBackground.M_BlackBackground"))

(fn `UserConstructionScript`
  (bind _sm_arcade_2 (`self.SM_Arcade-2`))
  ;[1 1 1] Random Mesh
  (switch `int` (`KismetMathLibrary.RandomIntegerInRange` 0 3)
    (:`0`
      (`StaticMeshComponent.SetStaticMesh` _sm_arcade_2 "/Game/BLAQ/Assets/Arcade-Machine/SM_Arcade-0.SM_Arcade-0"))
    (:`1`
      (`StaticMeshComponent.SetStaticMesh` _sm_arcade_2 "/Game/BLAQ/Assets/Arcade-Machine/SM_Arcade-1.SM_Arcade-1"))
    (:`2`
      (`StaticMeshComponent.SetStaticMesh` _sm_arcade_2 "/Game/BLAQ/Assets/Arcade-Machine/SM_Arcade-2.SM_Arcade-2"))
    (:`3`
      (`StaticMeshComponent.SetStaticMesh` _sm_arcade_2 "/Game/BLAQ/Assets/Arcade-Machine/SM_Arcade-3.SM_Arcade-3"))))