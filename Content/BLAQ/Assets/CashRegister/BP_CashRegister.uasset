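; Cash register actor that checks whether the player holds the required tickets when they interact with it.
; Binds to the first-person character's interact event, broadcasts on success, and sets the light and display to success or not-enough-tickets.
; The display is a dynamic material flipbook, with timelines driving frame offset and a helper swapping color and texture.
; A box trigger toggles a widget, and ending actor overlap restores the yellow waiting state.
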(event `self.ReceiveActorEndOverlap`
  (params (OtherActor :type "Actor Object Reference"))
  (`PrimitiveComponent.SetMaterial` (`self.Light`) 0 "/Game/BLAQ/Assets/CashRegister/MI_Yellow.MI_Yellow")
  (`self.SelectDisplayAnimation` 0)
  (bind (_direction _newtrack_0) (`Timeline|Timeline_0`)
    (:`Update`
      (`MaterialInstanceDynamic.SetScalarParameterValue` (`self.DisplayMat`) "FlipBookOffset" _newtrack_0))))

(event `CashRegister Interaction`
  (bind _light (`self.Light`))
  (bind _asbp_first_person_character (cast `/Game/FirstPerson/Blueprints/BP_FirstPersonCharacter` (stale `self.Box.OnComponentBeginOverlap` OtherActor)))
  (if (>= (`/Game/FirstPerson/Blueprints/BP_FirstPersonCharacter.Tickets` _asbp_first_person_character) (`self.RequiredTickets`))
    (`self.HasEnoughTickets`)
    (`self.SelectDisplayAnimation` 1)
    (`PrimitiveComponent.SetMaterial` _light 0 "/Game/BLAQ/Assets/CashRegister/MI_GreenLight.MI_GreenLight")
    (bind (_direction _newtrack_0) (`Timeline|Animation` :!via `PlayFromStart` :!label _label)
      (:`Update`
        (`MaterialInstanceDynamic.SetScalarParameterValue` (`self.DisplayMat`) "FlipBookOffset" _newtrack_0)))
    (else
      (`self.SelectDisplayAnimation` 2)
      (`PrimitiveComponent.SetMaterial` _light 0 "/Game/BLAQ/Assets/CashRegister/MI_RedLight.MI_RedLight")
      (goto _label :!via `PlayFromStart`))))

(event `self.Box.OnComponentBeginOverlap`
  (params (OverlappedComponent :type "PrimitiveComponent Object Reference") (OtherActor :type "Actor Object Reference") (OtherComp :type "PrimitiveComponent Object Reference") (OtherBodyIndex :type Integer) (bFromSweep :type Boolean) (SweepResult :type "HitResult Structure (by ref)"))
  (`SceneComponent.SetHiddenInGame` (`self.Widget`) false false))

(event `self.Box.OnComponentEndOverlap`
  (params (OverlappedComponent :type "PrimitiveComponent Object Reference") (OtherActor :type "Actor Object Reference") (OtherComp :type "PrimitiveComponent Object Reference") (OtherBodyIndex :type Integer))
  (`SceneComponent.SetHiddenInGame` (`self.Widget`) true false))

(event `self.ReceiveBeginPlay`
  (`|ExecutionSequence`
    (:`then_0`
      (bind _asbp_first_person_character (cast `/Game/FirstPerson/Blueprints/BP_FirstPersonCharacter` (`GameplayStatics.GetPlayerCharacter` 0)))
      (add `/Game/FirstPerson/Blueprints/BP_FirstPersonCharacter.InteractWithCashRegister` _asbp_first_person_character (delegate `CashRegister Interaction`)))
    (:`then_1`
      ;[1 1 1] Setup for display animation
      (bind _returnvalue (`KismetMaterialLibrary.CreateDynamicMaterialInstance` "/Game/BLAQ/Assets/CashRegister/M_CashRegisterDisplay.M_CashRegisterDisplay"))
      (bind _output_get (set `self.DisplayMat` _returnvalue))
      (`PrimitiveComponent.SetMaterial` (`self.SM_Register`) 2 _output_get))
    (:`then_2`
      (`self.SelectDisplayAnimation` 0)
      ;[1 1 1] Cant be in function sadly because timelines are not allowed :(
      (bind (_direction _newtrack_0) (`Timeline|Timeline`)
        (:`Update`
          (`MaterialInstanceDynamic.SetScalarParameterValue` (`self.DisplayMat`) "FlipBookOffset" _newtrack_0))))))

(fn `SelectDisplayAnimation`
  (params (NewParam :type Integer))
  (bind _displaymat (`self.DisplayMat`))
  (bind _displaymat_2 (`self.DisplayMat`))
  (switch `int` NewParam
    (:`0`
      (`MaterialInstanceDynamic.SetVectorParameterValue` _displaymat "Color" (struct :`R` 1.0 :`G` 0.75 :`A` 1.0))
      (`MaterialInstanceDynamic.SetTextureParameterValue` _displaymat_2 "Animation" "/Game/BLAQ/Assets/CashRegister/animations/Waiting.Waiting"))
    (:`1`
      (`MaterialInstanceDynamic.SetVectorParameterValue` _displaymat "Color" (struct :`G` 1.0 :`B` 0.029982 :`A` 1.0))
      (`MaterialInstanceDynamic.SetTextureParameterValue` _displaymat_2 "Animation" "/Game/BLAQ/Assets/CashRegister/animations/Success.Success"))
    (:`2`
      (`MaterialInstanceDynamic.SetVectorParameterValue` _displaymat "Color" (struct :`R` 1.0 :`A` 1.0))
      (`MaterialInstanceDynamic.SetTextureParameterValue` _displaymat_2 "Animation" "/Game/BLAQ/Assets/CashRegister/animations/NotEnoughTickets.NotEnoughTickets"))))

(fn `UserConstructionScript`)