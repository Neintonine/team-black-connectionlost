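; Arcade machine prop that varies its cabinet mesh and screen, and dims the screen on request.
; Construction picks one of three meshes from a location-seeded stream and records its screen material slot.
; BeginPlay uses a weighted roll to choose a dynamic CRT material with random image and color, or a disabled screen.
; DimLights swaps in an enemy-pass material, and BrightenLights restores the chosen one after a short delay.
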(event `self.ReceiveBeginPlay`
  (if (`KismetMathLibrary.RandomBoolWithWeight` (`self.DisplayArcade`))
    (bind _returnvalue (`PrimitiveComponent.CreateDynamicMaterialInstance` (`self.SM_Arcade-2`) (`self.ScreenIndex`) "/Game/CRT_VCR_Material/Materials/00_animated_crt_v2_1.00_animated_crt_v2_1" "None"))
    (`MaterialInstanceDynamic.SetTextureParameterValue` _returnvalue "Display Input" (`KismetArrayLibrary.Array_Random` (`self.ScreenImages`)))
    (`MaterialInstanceDynamic.SetVectorParameterValue` _returnvalue "Emissive color" (`KismetArrayLibrary.Array_Random` (`self.Colors`)))
    (set `self.Material` _returnvalue)
    (else
      (set `self.Material` "/Game/BLAQ/Assets/ArcadeMachines/Screen/Arcade/MI_Screen_Arcade_Disabled.MI_Screen_Arcade_Disabled")))
  (`PrimitiveComponent.SetMaterial` (`self.SM_Arcade-2`) (`self.ScreenIndex`) (`self.Material`) :!label _label))

(event `BrightenLights`
  (`KismetSystemLibrary.Delay` 0.2)
  (goto _label))

(event `DimLights`
  (`PrimitiveComponent.SetMaterial` (`self.SM_Arcade-2`) (`self.ScreenIndex`) "/Game/BLAQ/Assets/ArcadeMachines/Screen/Arcade/MI_Screen_Arcade_EnemyPass.MI_Screen_Arcade_EnemyPass"))

(fn `UserConstructionScript`
  (bind (_returnvalue_x _returnvalue_y _returnvalue_z) (`KismetMathLibrary.BreakVector` (`self.K2_GetActorLocation`)))
  (bind _sm_arcade_2 (`self.SM_Arcade-2`))
  ;[1 1 1] Random Mesh
  (switch `int` (`KismetMathLibrary.RandomIntegerInRangeFromStream` (`KismetMathLibrary.MakeRandomStream` (`KismetMathLibrary.FTrunc` (+ _returnvalue_x _returnvalue_y _returnvalue_z))) 0 2)
    (:`0`
      (`StaticMeshComponent.SetStaticMesh` _sm_arcade_2 "/Game/BLAQ/Assets/ArcadeMachines/ArcadeVariations/SM_arcadeMachine_01_b.SM_arcadeMachine_01_b")
      (set `self.ScreenIndex` 1))
    (:`1`
      (`StaticMeshComponent.SetStaticMesh` _sm_arcade_2 "/Game/BLAQ/Assets/ArcadeMachines/ArcadeVariations/SM_arcadeMachine_01_c.SM_arcadeMachine_01_c")
      (set `self.ScreenIndex` 1))
    (:`2`
      (`StaticMeshComponent.SetStaticMesh` _sm_arcade_2 "/Game/BLAQ/Assets/ArcadeMachines/ArcadeVariations/SM_arcadeMachine_01_e.SM_arcadeMachine_01_e")
      (set `self.ScreenIndex` 0))))