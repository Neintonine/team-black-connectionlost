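; Obstacle spawner for the Hopper arcade game that creates random obstacles at its arrow's transform.
; Each frame it polls a shared BPArcadeTicker, which gates spawning to a fixed tick interval, and picks a random class from SpawnableObstacles.
; Spawned Hopper obstacles receive the same ticker and an incrementing element index.
; It tracks every spawned actor and destroys those still valid on EndPlay.
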(event `self.ReceiveTick`
  (params (DeltaSeconds :type "Float (single-precision)"))
  (bind _allowed (`/Game/Devs/Michel/Blueprints/BP_ArcadeTicker.CheckTick` (`self.BP_ArcadeTicker`) 10 0))
  (if _allowed
    (set `self.SpawnedCount` (+ (`self.SpawnedCount`) 1))
    (bind _returnvalue (`|SpawnActorFromClass` (`KismetArrayLibrary.Array_Random` (`self.SpawnableObstacles`)) (`SceneComponent.K2_GetComponentToWorld` (`self.Arrow`)) "Undefined" "MultiplyWithRoot" null null))
    (`KismetArrayLibrary.Array_Add` (`self.SpawnedObstacles`) _returnvalue)
    (bind _asbp_hopper_obstacle (cast `/Game/Devs/Michel/Blueprints/Hopper/BP_HOPPER_Obstacle` _returnvalue))
    (set `/Game/Devs/Michel/Blueprints/Hopper/BP_HOPPER_Obstacle.Ticker` (`self.BP_ArcadeTicker`) _asbp_hopper_obstacle)
    (set `/Game/Devs/Michel/Blueprints/Hopper/BP_HOPPER_Obstacle.ElementIndex` (`self.SpawnedCount`) _asbp_hopper_obstacle)))

(event `self.ReceiveEndPlay`
  (params (EndPlayReason :type "EEndPlayReason Enum" :default "Destroyed"))
  (for _array_element (`self.SpawnedObstacles`)
    (if (`KismetSystemLibrary.IsValid` _array_element)
      (`self.K2_DestroyActor` _array_element))))

(fn `UserConstructionScript`)