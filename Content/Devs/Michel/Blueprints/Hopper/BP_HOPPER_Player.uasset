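; Player for the Hopper minigame, a Frogger-style game of hopping in grid steps toward targets while avoiding obstacles.
; Enhanced Input moves it forward or sideways within a horizontal limit; overlapping an obstacle or occupied target loses.
; A free target becomes occupied, then either the game is won or a display character spawns there and the player returns to its origin.
; Tick traces downward for obstacles but does nothing with the result.
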(event `self.ReceiveBeginPlay`
  (`parent.ReceiveBeginPlay`)
  (set `self.OriginPosition` (`SceneComponent.K2_GetComponentLocation` (`self.DefaultSceneRoot`))))

(event `EnhancedInput|/Game/Devs/Michel/Input/Actions/IA_HOPPER_Move`
  (params (ActionValue :type "Vector2D Structure") (ElapsedSeconds :type "Float (double-precision)") (TriggeredSeconds :type "Float (double-precision)") (InputAction :type "InputAction Object Reference" :default "/Game/Devs/Michel/Input/Actions/IA_HOPPER_Move.IA_HOPPER_Move"))
  (bind _returnvalue_x (`KismetMathLibrary.BreakVector` (`SceneComponent.K2_GetComponentLocation` (`self.DefaultSceneRoot`))))
  (bind _returnvalue (* (`/Game/Devs/Michel/Blueprints/BP_Arcade_Definitions.GetGridSize`) ActionValue_X))
  (:`Started`
    (`|ExecutionSequence`
      (:`then_0`
        (if (> ActionValue_Y 0.0)
          (`SceneComponent.K2_AddWorldOffset` (`self.DefaultSceneRoot`) (`KismetMathLibrary.MakeVector` 0.0 (* (`/Game/Devs/Michel/Blueprints/BP_Arcade_Definitions.GetGridSize`) -2.0)) false false)))
      (:`then_1`
        (if (> (`KismetMathLibrary.Abs` ActionValue_X) 0.1)
          (if (< (`KismetMathLibrary.Abs` (+ _returnvalue_x _returnvalue)) 500.0)
            (`SceneComponent.K2_AddWorldOffset` (`self.DefaultSceneRoot`) (`KismetMathLibrary.MakeVector` _returnvalue) false false))
          (set `self.RequestedDirection` 0.0))))))

(event `self.ReceiveActorBeginOverlap`
  (params (OtherActor :type "Actor Object Reference"))
  (`|ExecutionSequence`
    (:`then_0`
      (cast `/Game/Devs/Michel/Blueprints/Hopper/BP_HOPPER_Obstacle` OtherActor)
      (`self.LoseGame`))
    (:`then_1`
      (bind _asbp_hopper_target (cast `/Game/Devs/Michel/Blueprints/Hopper/BP_HOPPER_Target` OtherActor))
      (`self.CompleteRun` _asbp_hopper_target))))

(event `self.ReceiveTick`
  (params (DeltaSeconds :type "Float (single-precision)"))
  (bind _returnvalue (`SceneComponent.K2_GetComponentLocation` (`self.DefaultSceneRoot`)))
  (bind (_outhit _returnvalue_2) (`KismetSystemLibrary.LineTraceSingle` _returnvalue (+ _returnvalue (* (`KismetMathLibrary.Vector_Up`) -350.0)) "TraceTypeQuery1"))
  (if _returnvalue_2
    (cast `/Game/Devs/Michel/Blueprints/Hopper/BP_HOPPER_Obstacle` (`.HitActor` (`GameplayStatics.BreakHitResult` _outhit)))))

(fn `CompleteRun`
  (params (Target :type "/Game/Devs/Michel/Blueprints/Hopper/BP_HOPPER_Target Object Reference"))
  (if (`/Game/Devs/Michel/Blueprints/Hopper/BP_HOPPER_Target.Occupied` Target)
    (`self.LoseGame`)
    (else
      (set `/Game/Devs/Michel/Blueprints/Hopper/BP_HOPPER_Target.Occupied` true Target)
      (if (>= (`self.CurrentRun`) (`self.RunsToWin`))
        (`self.WinGame`)
        (else
          (set `self.CurrentRun` (+ (`self.CurrentRun`) 1))
          (bind _returnvalue (`|SpawnActorFromClass` "/Game/Devs/Michel/Blueprints/Hopper/BP_HOPPER_PlayerCharacter.BP_HOPPER_PlayerCharacter_C" (`self.GetTransform` Target) "Undefined" "MultiplyWithRoot" null null))
          (set `/Game/Devs/Michel/Blueprints/Hopper/BP_HOPPER_Target.DisplayedCharacter` _returnvalue Target)
          (`SceneComponent.K2_SetWorldLocation` (`self.DefaultSceneRoot`) (`self.OriginPosition`) false false))))))

(fn `UserConstructionScript`
  (`parent.UserConstructionScript`))