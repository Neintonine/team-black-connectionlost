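; BP_HOPPER_Obstacle is a moving obstacle for the Hopper game.
; Each Tick it offsets its root along its forward vector without sweeping, scaled by grid size, Speed and delta time.
; It destroys itself once it is more than a fixed distance from the Spawner it references, so that distance check alone ends its lifetime.
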(event `self.ReceiveTick`
  (params (DeltaSeconds :type "Float (single-precision)"))
  (`SceneComponent.K2_AddWorldOffset` (`self.DefaultSceneRoot`) (* (`SceneComponent.GetForwardVector` (`self.DefaultSceneRoot`)) (`/Game/Devs/Michel/Blueprints/BP_Arcade_Definitions.GetGridSize`) DeltaSeconds (`self.Speed`)) false false)
  (if (> (`KismetMathLibrary.VSize` (- (`SceneComponent.K2_GetComponentLocation` (`/Game/Devs/Michel/Blueprints/Hopper/BP_HOPPER_ObstacleSpawner.DefaultSceneRoot` (`self.Spawner`))) (`SceneComponent.K2_GetComponentLocation` (`self.DefaultSceneRoot`)))) 1200.0)
    (`self.K2_DestroyActor`)))

(fn `UserConstructionScript`)