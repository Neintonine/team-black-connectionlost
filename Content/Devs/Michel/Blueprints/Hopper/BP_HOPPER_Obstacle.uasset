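; Obstacle actor for the Hopper prototype that advances along its forward vector in discrete grid steps.
; Each frame it queries Ticker's CheckTick with a tick index offset by its ElementIndex.
; When the check passes, the root moves one grid cell as a world offset without sweeping, so the move itself does no collision check.
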(event `self.ReceiveTick`
  (params (DeltaSeconds :type "Float (single-precision)"))
  (bind _allowed (`/Game/Devs/Michel/Blueprints/BP_ArcadeTicker.CheckTick` (`self.Ticker`) 3 (+ 10 (`self.ElementIndex`))))
  (if _allowed
    (`SceneComponent.K2_AddWorldOffset` (`self.DefaultSceneRoot`) (* (`SceneComponent.GetForwardVector` (`self.DefaultSceneRoot`)) (`/Game/Devs/Michel/Blueprints/BP_Arcade_Definitions.GetGridSize`)) false false)))

(fn `UserConstructionScript`)