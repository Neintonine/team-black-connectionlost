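; Ball actor for a Breakout minigame that bounces around the XY plane, starting with a randomly angled direction toward negative Y.
; Tick moves it by a swept offset and flips each direction axis according to the impact normal.
; Target hits notify TargetSpawner of destruction, and death zone hits fail the level through Player.
; Hits on the paddle's negative-Y face steer the rebound by the ball's offset from the paddle center.
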(event `self.ReceiveBeginPlay`
  (set `self.MovementDirection` (`KismetMathLibrary.Normal` (`KismetMathLibrary.MakeVector` (`KismetMathLibrary.RandomFloatInRange` -0.75 0.75) -1.0))))

(event `self.ReceiveTick`
  (params (DeltaSeconds :type "Float (single-precision)"))
  (bind (_movementdirection_x _movementdirection_y) (`KismetMathLibrary.BreakVector` (`self.MovementDirection`)))
  (bind _returnvalue_x (`KismetMathLibrary.BreakVector` (`SceneComponent.K2_GetComponentLocation` (`self.SphereCollision`))))
  (bind _sweephitresult (`SceneComponent.K2_AddWorldOffset` (`self.SphereCollision`) (* DeltaSeconds (`self.Speed`) (`self.MovementDirection`)) true false))
  (bind (_bblockinghit _binitialoverlap _time _distance _location _impactpoint _normal _impactnormal _physmat _hitactor) (`GameplayStatics.BreakHitResult` _sweephitresult))
  (if _bblockinghit
    (`|ExecutionSequence`
      (:`then_0`
        (if (> (`KismetMathLibrary.Abs` (.x _impactnormal)) 0.1)
          (set `self.MovementDirection` (* (`self.MovementDirection`) (-1.0 1.0 1.0)))))
      (:`then_1`
        (if (> (`KismetMathLibrary.Abs` (.y _impactnormal)) 0.1)
          (set `self.MovementDirection` (* (`self.MovementDirection`) (1.0 -1.0 1.0)))))
      (:`then_2`
        (bind _asbp_breakout_target (cast `/Game/Devs/Michel/Blueprints/Breakout/BP_BREAKOUT_Target` _hitactor))
        (`/Game/Devs/Michel/Blueprints/Breakout/BP_BREAKOUT_TargetSpawner.NotifyDestroy` (`self.TargetSpawner`) _asbp_breakout_target))
      (:`then_3`
        (cast `/Game/Devs/Michel/Blueprints/Breakout/BP_BREAKOUT_DeathZone` _hitactor)
        (`/Game/Devs/Michel/Blueprints/BP_ArcadePlayer.FailLevel` (`self.Player`)))
      (:`then_4`
        (bind _asbp_breakout_player (cast `/Game/Devs/Michel/Blueprints/Breakout/BP_BREAKOUT_Player` _hitactor))
        (if (> (`KismetMathLibrary.Dot_VectorVector` _impactnormal (0.0 -1.0 0.0)) 0.9)
          (bind _returnvalue_x_2 (`KismetMathLibrary.BreakVector` (`SceneComponent.K2_GetComponentLocation` (`/Game/Devs/Michel/Blueprints/BP_ArcadePlayer.DefaultSceneRoot` _asbp_breakout_player))))
          (bind _returnvalue_x_3 (`KismetMathLibrary.BreakVector` (`BoxComponent.GetScaledBoxExtent` (`/Game/Devs/Michel/Blueprints/Breakout/BP_BREAKOUT_Player.Box` _asbp_breakout_player))))
          (set `self.MovementDirection` (`KismetMathLibrary.Normal` (`KismetMathLibrary.MakeVector` (`KismetMathLibrary.Lerp` 0.0 0.75 (/ (- _returnvalue_x _returnvalue_x_2) _returnvalue_x_3)) _movementdirection_y))))))))

(fn `UserConstructionScript`)