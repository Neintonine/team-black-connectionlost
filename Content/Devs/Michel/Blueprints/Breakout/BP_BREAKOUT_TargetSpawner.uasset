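; Breakout target spawner actor that builds the brick grid for a level and tracks when it is cleared.
; On BeginPlay it spawns BP_BREAKOUT_Target actors in rows and columns sized by Grid, offset from its root, and cycles Materials per row.
; NotifyDestroy removes and destroys a target, then calls CompleteLevel on Player once none remain.
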(event `self.ReceiveBeginPlay`
  (bind (_grid_x _grid_y) (`KismetMathLibrary.BreakVector2D` (`self.Grid`)))
  (for _index (range (`KismetMathLibrary.FTrunc` _grid_y))
    (for _index_2 (range (`KismetMathLibrary.FTrunc` _grid_x))
      (bind _returnvalue (`|SpawnActorFromClass` "/Game/Devs/Michel/Blueprints/Breakout/BP_BREAKOUT_Target.BP_BREAKOUT_Target_C" (`KismetMathLibrary.MakeTransform` (+ (`KismetMathLibrary.MakeVector` (* _index_2 100) (* _index -25)) (`SceneComponent.K2_GetComponentLocation` (`self.DefaultSceneRoot`)))) "Undefined" "MultiplyWithRoot" self null))
      (`KismetArrayLibrary.Array_Add` (`self.SpawnedTargets`) _returnvalue)
      (`PrimitiveComponent.SetMaterial` (`/Game/Devs/Michel/Blueprints/Breakout/BP_BREAKOUT_Target.Cube` _returnvalue) 0 (`|GetArrayItem` (`self.Materials`) (mod _index (`KismetArrayLibrary.Array_Length` (`self.Materials`))))))))

(fn `NotifyDestroy`
  (params (`Target Object` :type "/Game/Devs/Michel/Blueprints/Breakout/BP_BREAKOUT_Target Object Reference"))
  (`KismetArrayLibrary.Array_RemoveItem` (`self.SpawnedTargets`) `Target Object`)
  (`self.K2_DestroyActor` `Target Object`)
  (if (< (`KismetArrayLibrary.Array_Length` (`self.SpawnedTargets`)) 1)
    (`/Game/Devs/Michel/Blueprints/BP_ArcadePlayer.CompleteLevel` (`self.Player`))))

(fn `UserConstructionScript`)