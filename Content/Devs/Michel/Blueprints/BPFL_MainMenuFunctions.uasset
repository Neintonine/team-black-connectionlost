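; Blueprint function library that opens and closes the main menu widget for the first local player.
; OpenMainMenu creates BP_UI_MainMenu on a chosen switcher page, shows it with the cursor and game-and-UI input focused on it, optionally pauses, and returns the widget.
; CloseMainMenu removes the given widget, always unpauses, and restores game-only input with a hidden cursor if the player controller is valid.
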(fn `CloseMainMenu`
  (params (Target :type "Widget Object Reference"))
  (bind _returnvalue (`GameplayStatics.GetPlayerController` null))
  (`Widget.RemoveFromParent` Target)
  (`GameplayStatics.SetGamePaused` null)
  (`/Engine/EditorBlueprintResources/StandardMacros.IsValid` _returnvalue
    (:`Is Valid`
      (`WidgetBlueprintLibrary.SetInputMode_GameOnly` _returnvalue)
      (set `PlayerController.bShowMouseCursor` false _returnvalue))))

(fn `OpenMainMenu`
  (params (Index :type Integer) (AllowPause :type Boolean :default true))
  (returns (Widget :type "/Game/BLAQ/Blueprints/BP_UI_MainMenu Object Reference"))
  (bind _returnvalue (`|CreateWidget` "/Game/BLAQ/Blueprints/BP_UI_MainMenu.BP_UI_MainMenu_C"))
  (`WidgetSwitcher.SetActiveWidgetIndex` (`/Game/BLAQ/Blueprints/BP_UI_MainMenu.WidgetSwitcherUI` _returnvalue) Index)
  (`UserWidget.AddToViewport` _returnvalue 0)
  (`WidgetBlueprintLibrary.SetInputMode_GameAndUIEx` (`GameplayStatics.GetPlayerController` null) _returnvalue)
  (set `PlayerController.bShowMouseCursor` true (`GameplayStatics.GetPlayerController` null))
  (if AllowPause
    (`GameplayStatics.SetGamePaused` null true))
  (return _returnvalue))