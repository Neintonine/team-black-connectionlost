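; Main menu spawner that keeps a single BP_MainMenu_Enemy on show, replacing it on a repeating timer.
; BeginPlay spawns the first enemy at once, and each timer tick destroys the previous one before spawning the next.
; A weighted coin flip occasionally places it just in front of the MenuPawn camera, otherwise at a random point in a fixed distant plane.
; Its spawn rotation faces the MenuPawn.
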(event `self.ReceiveBeginPlay`
  (bind _returnvalue (`KismetMathLibrary.SelectVector` (+ (* 250.0 (`SceneComponent.GetForwardVector` (`/Game/Devs/Michel/Blueprints/MainMenu/BP_MainMenuPawn.Camera` (`self.MenuPawn`)))) (`SceneComponent.K2_GetComponentLocation` (`/Game/Devs/Michel/Blueprints/MainMenu/BP_MainMenuPawn.Camera` (`self.MenuPawn`)))) (`KismetMathLibrary.MakeVector` 2500.0 (`KismetMathLibrary.RandomFloatInRange` -1000.0 1000.0) (`KismetMathLibrary.RandomFloatInRange` -500.0 500.0)) (`KismetMathLibrary.RandomBoolWithWeight` 0.1)))
  (`KismetSystemLibrary.K2_SetTimerDelegate` (delegate `Spawn`) 5.0 true)
  (`/Engine/EditorBlueprintResources/StandardMacros.IsValid` (`self.OldEnemy`) :!label _label
    (:`Is Valid`
      (`self.K2_DestroyActor` (`self.OldEnemy`)))
    (:`Is Not Valid`
      _))
  (bind _returnvalue_2 (`|SpawnActorFromClass` "/Game/Devs/Michel/Blueprints/MainMenu/BP_MainMenu_Enemy.BP_MainMenu_Enemy_C" (`KismetMathLibrary.MakeTransform` _returnvalue (`KismetMathLibrary.FindLookAtRotation` _returnvalue (`self.K2_GetActorLocation` (`self.MenuPawn`)))) "Undefined" "MultiplyWithRoot" self null))
  (set `self.OldEnemy` _returnvalue_2))

(event `Spawn`
  (goto _label))

(fn `UserConstructionScript`)