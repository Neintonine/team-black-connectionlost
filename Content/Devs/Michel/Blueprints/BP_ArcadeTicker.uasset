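; BP_ArcadeTicker turns frame time into a counted tick, apparently for arcade-style stepped updates.
; Tick accumulates delta time; past the GetFramerate threshold, it increments CurrentTick, clears InvokedTicks and sets the time to threshold minus accumulated, going negative and ending the loop after one pass.
; CheckTick returns true once per index on ticks divisible by the requested difference, using InvokedTicks to block repeats.
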(event `self.ReceiveTick`
  (params (DeltaSeconds :type "Float (single-precision)"))
  (set `self.CurrentTime` (+ DeltaSeconds (`self.CurrentTime`)))
  (if (> (`self.CurrentTime`) (`/Game/Devs/Michel/Blueprints/BP_Arcade_Definitions.GetFramerate`))
    (while (> (`self.CurrentTime`) (`/Game/Devs/Michel/Blueprints/BP_Arcade_Definitions.GetFramerate`))
      (set `self.CurrentTime` (- (`/Game/Devs/Michel/Blueprints/BP_Arcade_Definitions.GetFramerate`) (`self.CurrentTime`)))
      (set `self.CurrentTick` (+ (`self.CurrentTick`) 1))
      (`KismetArrayLibrary.Array_Clear` (`self.InvokedTicks`)))))

(fn `CheckTick`
  (params (`Tick Difference` :type Integer :default 1) (`Tick Index` :type Integer))
  (returns (Allowed :type Boolean))
  (if (`KismetArrayLibrary.Array_Contains` (`self.InvokedTicks`) `Tick Index`)
    (return false)
    (elif (== (mod (`self.CurrentTick`) `Tick Difference`) 0)
      (`KismetArrayLibrary.Array_Add` (`self.InvokedTicks`) `Tick Index`)
      (return true)
      (else
        (return false)))))