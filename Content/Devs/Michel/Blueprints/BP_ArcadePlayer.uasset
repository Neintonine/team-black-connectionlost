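; BP_ArcadePlayer is the player-possessed actor used during an arcade machine game, apparently a base for minigame players.
; On BeginPlay it takes possession from the first-person character, keeps the camera view on that character and adds its input mapping context.
; Setup stores the owning arcade machine, which receives the exit input and LoseGame as ExitArcade, and WinGame as a win with a fixed value.
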(event `self.ReceiveBeginPlay`
  (bind _returnvalue (`GameplayStatics.GetPlayerController` 0))
  (bind _asbp_first_person_character (cast `/Game/FirstPerson/Blueprints/BP_FirstPersonCharacter` (`GameplayStatics.GetPlayerCharacter` 0)))
  (set `self.ActualPlayerCharacter` _asbp_first_person_character)
  (`Controller.Possess` _returnvalue self)
  (`PlayerController.SetViewTargetWithBlend` _returnvalue (`self.ActualPlayerCharacter`) 0.0 "VTBlend_Linear" 0.0 false)
  (`EnhancedInputSubsystemInterface.AddMappingContext` (pcsubsystem `EnhancedInputLocalPlayerSubsystem` (`GameplayStatics.GetPlayerController` 0)) (`self.InputMapping`) 0 (struct)))

(event `EnhancedInput|/Game/Devs/Michel/Input/Actions/IA_ExitArcade`
  (params (ActionValue :type Boolean) (ElapsedSeconds :type "Float (double-precision)") (TriggeredSeconds :type "Float (double-precision)") (InputAction :type "InputAction Object Reference" :default "/Game/Devs/Michel/Input/Actions/IA_ExitArcade.IA_ExitArcade"))
  (:`Triggered`
    (`/Game/Devs/Michel/Blueprints/BP_PlayableArcade.ExitArcade` (`self.ArcadeMachine`))))

(fn `LoseGame`
  (`/Game/Devs/Michel/Blueprints/BP_PlayableArcade.ExitArcade` (`self.ArcadeMachine`)))

(fn `Setup`
  (params (ArcadeMachine :type "/Game/Devs/Michel/Blueprints/BP_PlayableArcade Object Reference"))
  (bind _output_get (set `self.ArcadeMachine` ArcadeMachine)))

(fn `UserConstructionScript`)

(fn `WinGame`
  (`/Game/Devs/Michel/Blueprints/BP_PlayableArcade.WinGame` (`self.ArcadeMachine`) 5))