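; BP_CashRegister is a cash register actor that shows whether the player holds enough tickets.
; When a BP_FirstPersonCharacter begins overlapping it, it compares the character's Tickets to its required amount and sets the Index component's material to green or red.
; Any end overlap switches the material to yellow, and no tickets are deducted.
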(event `self.ReceiveActorBeginOverlap`
  (params (OtherActor :type "Actor Object Reference"))
  (bind _asbp_first_person_character (cast `/Game/FirstPerson/Blueprints/BP_FirstPersonCharacter` OtherActor))
  (if (>= (`/Game/FirstPerson/Blueprints/BP_FirstPersonCharacter.Tickets` _asbp_first_person_character) (`self.Required ickets`))
    (`PrimitiveComponent.SetMaterial` (`self.Index`) 0 "/Game/Devs/Fynn/Cash_Register/MI_GreenLight.MI_GreenLight")
    (else
      (`PrimitiveComponent.SetMaterial` (`self.Index`) 0 "/Game/Devs/Fynn/Cash_Register/MI_RedLight.MI_RedLight"))))

(event `self.ReceiveActorEndOverlap`
  (params (OtherActor :type "Actor Object Reference"))
  (`PrimitiveComponent.SetMaterial` (`self.Index`) 0 "/Game/Devs/Fynn/Cash_Register/MI_Yellow.MI_Yellow"))

(fn `UserConstructionScript`)