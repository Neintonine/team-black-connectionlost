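; BP_SlideDoor is a two-part sliding door in a dev level that opens through a DoorOpener event and closes when an actor overlap ends.
; A timeline's DoorOpen track, scaled by DoorDistance, slides the Arrow1 and Arrow components in opposite directions along X, playing forward to open and reversing to close.
; The construction script places both at full open offset, and BeginPlay resets their relative locations.
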(event `DoorOpener`
  (bind (_direction _dooropen) (`Timeline|Timeline` :!label _label)
    (:`Update`
      (`|ExecutionSequence`
        (:`then_0`
          (bind _returnvalue (* _dooropen (`self.DoorDistance`)))
          (`SceneComponent.K2_SetRelativeLocation` (`self.Arrow1`) (`KismetMathLibrary.MakeVector` _returnvalue) false false))
        (:`then_1`
          (`SceneComponent.K2_SetRelativeLocation` (`self.Arrow`) (`KismetMathLibrary.MakeVector` (* _returnvalue -1.0)) false false))))))

(event `self.ReceiveActorEndOverlap`
  (params (OtherActor :type "Actor Object Reference"))
  (goto _label :!via `Reverse`))

(event `self.ReceiveBeginPlay`
  (`SceneComponent.K2_SetRelativeLocation` (`self.Arrow1`) (0.0 0.0 0.0) false false)
  (`SceneComponent.K2_SetRelativeLocation` (`self.Arrow`) (0.0 0.0 0.0) false false))

(fn `UserConstructionScript`
  (bind _doordistance (`self.DoorDistance`))
  (`|ExecutionSequence`
    (:`then_0`
      (`SceneComponent.K2_SetRelativeLocation` (`self.Arrow1`) (`KismetMathLibrary.MakeVector` _doordistance) false false))
    (:`then_1`
      (`SceneComponent.K2_SetRelativeLocation` (`self.Arrow`) (`KismetMathLibrary.MakeVector` (* _doordistance -1.0)) false false))))